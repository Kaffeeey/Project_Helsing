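; Interactive dungeon lever actor that the player toggles with the E key while inside its front trigger.
; Trigger overlap enables input and opens a gate; leaving it disables input.
; Each press flips DoorState and plays the LeverR timeline forward or in reverse, rotating the lever's roll offset by the construction-time actor rotation.
; A Moving flag, cleared after a delay from timeline updates, blocks repeat presses.
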(event `Key|E`
  (params (Key :type "Key Structure"))
  (bind _initrot_roll (`KismetMathLibrary.BreakRotator` (`self.InitRot`)))
  (:`Pressed`
    (`/Engine/EditorBlueprintResources/StandardMacros.Gate` true :!label _label
      (:`Exit`
        (if (not (`self.Moving`))
          (set `self.Moving` true)
          (switch `int` (`self.DoorState`)
            (:`0`
              (set `self.DoorState` 1)
              (bind (_direction _leverr) (`Timeline|leverR` :!via `PlayFromStart` :!label _label_2)
                (:`Update`
                  (`SceneComponent.K2_SetRelativeRotation` (`self.Lever`) (`KismetMathLibrary.MakeRotator` (+ _leverr _initrot_roll)) false false)
                  (`KismetSystemLibrary.Delay` 2.0)
                  (set `self.Moving` false))))
            (:`1`
              (set `self.DoorState` 0)
              (goto _label_2 :!via `ReverseFromEnd`))))))))

(event `self.TriggerFront.OnComponentBeginOverlap`
  (params (OverlappedComponent :type "PrimitiveComponent Object Reference") (OtherActor :type "Actor Object Reference") (OtherComp :type "PrimitiveComponent Object Reference") (OtherBodyIndex :type Integer) (bFromSweep :type Boolean) (SweepResult :type "HitResult Structure (by ref)"))
  (`self.EnableInput` (`GameplayStatics.GetPlayerController` 0))
  (goto _label :!via `Open`))

(event `self.TriggerFront.OnComponentEndOverlap`
  (params (OverlappedComponent :type "PrimitiveComponent Object Reference") (OtherActor :type "Actor Object Reference") (OtherComp :type "PrimitiveComponent Object Reference") (OtherBodyIndex :type Integer))
  (`self.DisableInput` (`GameplayStatics.GetPlayerController` 0)))

(fn `UserConstructionScript`
  (bind _returnvalue (`self.K2_GetActorRotation`))
  (`self.K2_SetActorRotation` _returnvalue)
  (set `self.InitRot` _returnvalue))