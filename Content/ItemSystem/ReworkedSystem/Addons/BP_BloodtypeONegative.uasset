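; BP_BloodtypeONegative is an interactable item addon that permanently removes itself on pickup and raises the player's healing per potion.
; On interact, it runs the parent item logic, then adds its HealingPerFlask value to the player's HPGain through a small addition helper function.
; The actor destroys itself after applying the bonus.
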(event `/Game/Inventory/Interact_Interface.ItemInteract`
  (params (Interactor :type "Actor Object Reference"))
  (`parent.ItemInteract` Interactor)
  (bind _newparam (`self.GetPlayer`))
  (bind _newhp_perpotion (`self.HP Per Potion` (`/Game/Blueprints/FPSChar_V_0_3.HPGain` _newparam) (`self.HealingPerFlask`)))
  (set `/Game/Blueprints/FPSChar_V_0_3.HPGain` _newhp_perpotion _newparam)
  (`self.K2_DestroyActor`))

(fn `HP Per Potion`
  (params (`CurrentHP PerPotion` :type "Float (double-precision)") (`AddedHP PerPotion` :type "Float (double-precision)"))
  (returns (`NewHP PerPotion` :type "Float (double-precision)"))
  (return (+ `CurrentHP PerPotion` `AddedHP PerPotion`)))

(fn `UserConstructionScript`
  (`parent.UserConstructionScript`))