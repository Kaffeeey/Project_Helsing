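; Weapon addon pickup, Helsing's Magazine, that enlarges the clip of the player's gun when interacted with.
; On interact it saves the current gun, rewrites the first GunArray entry through ChangeClipSize, rebuilds the weapon and destroys itself.
; ChangeClipSize copies the gun struct with AddClipSize added and appends bullet entries in a fixed-count loop, independent of AddClipSize.
; NewFunction_0 is an uncalled struct-copy helper.
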(event `/Game/Inventory/Interact_Interface.ItemInteract`
  (params (Interactor :type "Actor Object Reference"))
  (`parent.ItemInteract` Interactor)
  (bind _newparam (`self.GetPlayer`))
  (bind _asgun_parent (cast `/Game/FirstPersonBP/Blueprints/Guns/Gun_Parent` (`ChildActorComponent.ChildActor` (`/Game/Blueprints/FPSChar_V_0_3.Gun` _newparam))))
  (`/Game/Blueprints/FPSChar_V_0_3.SaveCurrentGun` _newparam)
  (bind _output (`|GetArrayItem` (`/Game/Blueprints/FPSChar_V_0_3.GunArray` _newparam)))
  (bind _newgun (`self.Change Clip Size` _output (`self.AddClipSize`) _asgun_parent))
  (`|VariableSetRef` _output _newgun)
  (`/Game/Blueprints/FPSChar_V_0_3.BuildWeapon` _newparam)
  (`self.K2_DestroyActor`))

(fn `Change Clip Size`
  (params (Gun :type "/Game/FirstPersonBP/Blueprints/Guns/GunVariables Structure") (AddClipSize :type Integer) (NewParam :type "/Game/FirstPersonBP/Blueprints/Guns/Gun_Parent Object Reference"))
  (returns (NewGun :type "/Game/FirstPersonBP/Blueprints/Guns/GunVariables Structure"))
  (locals (Bullets2 :type "Array of /Game/FirstPersonBP/Blueprints/Guns/Bullet Structure"))
  (for _ (range 3)
    (`KismetArrayLibrary.Array_Add` Gun_Bullets_32_94AD3E4E46EB673342C43EB25F42E653 (make `/Game/FirstPersonBP/Blueprints/Guns/Bullet` false true)))
  (return (make `/Game/FirstPersonBP/Blueprints/Guns/GunVariables` Gun_GunType_2_14FC35544E58478CA236669C8A25613F Gun_AmmoCurrent_5_5302FF684AA84A1D4269D996DDF371EA Gun_AmmoMax_7_5F39C5A345B67AEE2D137699778EDCFD Gun_BulletAngle_13_BFD283954948BD292AA064BFA0F8E516 Gun_Damage_17_99EB532E4ED9FC782950138E04B2F512 (+ Gun_ClipSize_20_3B0274BE43EBE86114EAD6A682365631 AddClipSize) Gun_DamageAmp_25_734A8F6241C66E18F8506C9CDF54D76E Gun_ClipCount_28_66C030C441DA950025982B936A504732 Gun_Bullets_32_94AD3E4E46EB673342C43EB25F42E653 Gun_BoltType_36_F8ADBC2D4954BBB8298E108193B2078D Gun_MaxAmmoLimit_39_E9180C084BC0FD87DC0099BE96B5F6C7 Gun_KnockbackStrengthMultiplier_43_5DF9E7DC44733A2B82F379BAACE4A378 Gun_ReloadTimeReduction_46_764E97C24ED54D09720A80BF7A086918 Gun_ReloadOnSwap_49_5273A4EB49D327EAD27B7EA53FFEB553 Gun_CritMultiplier_54_FD153910476009D858F2EF8FA7CD60ED Gun_PiercingBullets_52_F919B5B7494EBC48894AEAB37D83D932 Gun_CritChance_57_6C7773F1480E01B5C401CC94A9B11E98 Gun_AmmoOnCrit_83_DF1B68634193D27A4D5473BC552235F8 Gun_GoldenChance_63_F512CEC843A90B444CA310AC5EF4EE5E Gun_ReloadWeaponOnHit_68_3498DF844B1A89273EC82BA630D9EB01 Gun_StunOnHit_69_23E8D78D4D5712661930D58EEECD3E84 Gun_BloodOnCrit_82_5A55CE534D8E6E07EF7B7BBB2E920952 Gun_NearbyDamageOnCrit_81_2DEDA9ED4855CBC0A820DFA7292A1EA3 Gun_LastBulletDamage_80_1D69B9EE4F228D3E5AE782A956DCA5D6 Gun_CashOnCrit_89_501F8B734C5439FC0B98DDBD6FB96B72 Gun_BloodOnArealKill_91_4088028046EF146BAA56FC93122D04C3 Gun_HealOnEnemyKill_94_13C4736D47C3BF73488A1B87D406C2E1 Gun_ReduceCDsOnKill_96_18AAEC864D5AFDF9092A6F839BDFEC25 Gun_ParalyzeDuration_99_529C116E4621F07F03175491E73C062D Gun_RevolvoDropChance_106_9E8A31844667725DA4FDF8B8EB678097 Gun_ShotgunDropChance_107_C66A95BC4EDC52418AD40E8DF6471FC8 Gun_CrossbowDropChance_108_E43373764BD32B81E807E0B5285796A8 Gun_HPDropChance_110_77F2D1A44D586FAB59D1B2B3DA6032D1)))

(fn `NewFunction_0`
  (params (Gun :type "/Game/FirstPersonBP/Blueprints/Guns/GunVariables Structure") (NewParam1 :type "Array of /Game/FirstPersonBP/Blueprints/Guns/Bullet Structure (by ref)") (Gun_GunType :type "/Game/FirstPersonBP/Blueprints/Guns/Gun_Parent Class Reference") (Gun_AmmoCurrent :type Integer) (Gun_AmmoMax :type Integer) (Gun_BulletAngle :type "Float (double-precision)") (Gun_Damage :type "Float (double-precision)") (Gun_ClipSize :type Integer) (Gun_DamageAmp :type "Float (double-precision)") (Gun_ClipCount :type Integer) (Gun_Bullets :type "Array of /Game/FirstPersonBP/Blueprints/Guns/Bullet Structure") (Gun_BoltType :type "Actor Class Reference") (Gun_MaxAmmoLimit :type Integer) (Gun_KnockbackStrengthMultiplier :type "Float (double-precision)") (Gun_ReloadTimeReduction :type "Float (double-precision)") (Gun_ReloadOnSwap :type Boolean) (Gun_CritMultiplier :type "Float (double-precision)") (Gun_PiercingBullets :type Boolean) (Gun_CritChance :type "Float (double-precision)") (Gun_AmmoOnCrit :type "Float (double-precision)") (Gun_GoldenChance :type "Float (double-precision)") (Gun_ReloadWeaponOnHit :type Boolean) (Gun_StunOnHit :type Boolean) (Gun_BloodOnCrit :type "Float (double-precision)") (Gun_NearbyDamageOnCrit :type "Float (double-precision)") (Gun_LastBulletDamage :type "Float (double-precision)") (Gun_CashOnCrit :type Boolean) (Gun_BloodOnArealKill :type Boolean) (Gun_HealOnEnemyKill :type "Float (double-precision)") (Gun_ReduceCDsOnKill :type "Float (double-precision)") (Gun_ParalyzeDuration :type "Float (double-precision)") (Gun_RevolvoDropChance :type "Float (double-precision)") (Gun_ShotgunDropChance :type "Float (double-precision)") (Gun_CrossbowDropChance :type "Float (double-precision)") (Gun_HPDropChance :type "Float (double-precision)"))
  (returns (newGun :type "/Game/FirstPersonBP/Blueprints/Guns/GunVariables Structure") (newGun_GunType :type "/Game/FirstPersonBP/Blueprints/Guns/Gun_Parent Class Reference") (newGun_AmmoCurrent :type Integer) (newGun_AmmoMax :type Integer) (newGun_BulletAngle :type "Float (double-precision)") (newGun_Damage :type "Float (double-precision)") (newGun_ClipSize :type Integer) (newGun_DamageAmp :type "Float (double-precision)") (newGun_ClipCount :type Integer) (newGun_Bullets :type "Array of /Game/FirstPersonBP/Blueprints/Guns/Bullet Structure") (newGun_BoltType :type "Actor Class Reference") (newGun_MaxAmmoLimit :type Integer) (newGun_KnockbackStrengthMultiplier :type "Float (double-precision)") (newGun_ReloadTimeReduction :type "Float (double-precision)") (newGun_ReloadOnSwap :type Boolean) (newGun_CritMultiplier :type "Float (double-precision)") (newGun_PiercingBullets :type Boolean) (newGun_CritChance :type "Float (double-precision)") (newGun_AmmoOnCrit :type "Float (double-precision)") (newGun_GoldenChance :type "Float (double-precision)") (newGun_ReloadWeaponOnHit :type Boolean) (newGun_StunOnHit :type Boolean) (newGun_BloodOnCrit :type "Float (double-precision)") (newGun_NearbyDamageOnCrit :type "Float (double-precision)") (newGun_LastBulletDamage :type "Float (double-precision)") (newGun_CashOnCrit :type Boolean) (newGun_BloodOnArealKill :type Boolean) (newGun_HealOnEnemyKill :type "Float (double-precision)") (newGun_ReduceCDsOnKill :type "Float (double-precision)") (newGun_ParalyzeDuration :type "Float (double-precision)") (newGun_RevolvoDropChance :type "Float (double-precision)") (newGun_ShotgunDropChance :type "Float (double-precision)") (newGun_CrossbowDropChance :type "Float (double-precision)") (newGun_HPDropChance :type "Float (double-precision)"))
  (return (make `/Game/FirstPersonBP/Blueprints/Guns/GunVariables` Gun_GunType_2_14FC35544E58478CA236669C8A25613F Gun_AmmoCurrent_5_5302FF684AA84A1D4269D996DDF371EA Gun_AmmoMax_7_5F39C5A345B67AEE2D137699778EDCFD Gun_BulletAngle_13_BFD283954948BD292AA064BFA0F8E516 Gun_Damage_17_99EB532E4ED9FC782950138E04B2F512 Gun_ClipSize_20_3B0274BE43EBE86114EAD6A682365631 Gun_DamageAmp_25_734A8F6241C66E18F8506C9CDF54D76E Gun_ClipCount_28_66C030C441DA950025982B936A504732 NewParam1 Gun_BoltType_36_F8ADBC2D4954BBB8298E108193B2078D Gun_MaxAmmoLimit_39_E9180C084BC0FD87DC0099BE96B5F6C7 Gun_KnockbackStrengthMultiplier_43_5DF9E7DC44733A2B82F379BAACE4A378 Gun_ReloadTimeReduction_46_764E97C24ED54D09720A80BF7A086918 Gun_ReloadOnSwap_49_5273A4EB49D327EAD27B7EA53FFEB553 Gun_CritMultiplier_54_FD153910476009D858F2EF8FA7CD60ED Gun_PiercingBullets_52_F919B5B7494EBC48894AEAB37D83D932 Gun_CritChance_57_6C7773F1480E01B5C401CC94A9B11E98 Gun_AmmoOnCrit_83_DF1B68634193D27A4D5473BC552235F8 Gun_GoldenChance_63_F512CEC843A90B444CA310AC5EF4EE5E Gun_ReloadWeaponOnHit_68_3498DF844B1A89273EC82BA630D9EB01 Gun_StunOnHit_69_23E8D78D4D5712661930D58EEECD3E84 Gun_BloodOnCrit_82_5A55CE534D8E6E07EF7B7BBB2E920952 Gun_NearbyDamageOnCrit_81_2DEDA9ED4855CBC0A820DFA7292A1EA3 Gun_LastBulletDamage_80_1D69B9EE4F228D3E5AE782A956DCA5D6 Gun_CashOnCrit_89_501F8B734C5439FC0B98DDBD6FB96B72 Gun_BloodOnArealKill_91_4088028046EF146BAA56FC93122D04C3 Gun_HealOnEnemyKill_94_13C4736D47C3BF73488A1B87D406C2E1 Gun_ReduceCDsOnKill_96_18AAEC864D5AFDF9092A6F839BDFEC25 Gun_ParalyzeDuration_99_529C116E4621F07F03175491E73C062D Gun_RevolvoDropChance_106_9E8A31844667725DA4FDF8B8EB678097 Gun_ShotgunDropChance_107_C66A95BC4EDC52418AD40E8DF6471FC8 Gun_CrossbowDropChance_108_E43373764BD32B81E807E0B5285796A8 Gun_HPDropChance_110_77F2D1A44D586FAB59D1B2B3DA6032D1) null 0 0 0.0 0.0 0 0.0 0 _ null 0 0.0 0.0 false 0.0 false 0.0 0.0 0.0 false false 0.0 0.0 0.0 false false 0.0 0.0 0.0 0.0 0.0 0.0 0.0))

(fn `UserConstructionScript`
  (`parent.UserConstructionScript`))