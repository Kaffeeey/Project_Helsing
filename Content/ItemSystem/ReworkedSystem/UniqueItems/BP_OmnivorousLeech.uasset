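; BP_OmnivorousLeech is a unique item pickup that, on interaction, targets the player's gun slots with blood-on-crit and ammo-on-crit bonuses.
; It loops over GunArray, saving the current gun, chaining AddBloodOnCrit into AmmoOnCrit, writing the result back by reference and rebuilding the weapon each pass.
; Both helper functions contain only a return, with no visible stat logic.
; The actor destroys itself afterwards.
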(event `/Game/Inventory/Interact_Interface.ItemInteract`
  (params (Interactor :type "Actor Object Reference"))
  (`parent.ItemInteract` Interactor)
  (bind _newparam (`self.GetPlayer`))
  (for _index (range 3)
    (`/Game/Blueprints/FPSChar_V_0_3.SaveCurrentGun` _newparam)
    (bind _output (`|GetArrayItem` (`/Game/Blueprints/FPSChar_V_0_3.GunArray` _newparam) _index))
    (bind _newgun (`self.Add Blood on Crit` _output (`self.Blood on Crit`)))
    (bind _newgun_2 (`self.Ammo on Crit` _newgun (`self.AmmoOnCrit`)))
    (`|VariableSetRef` _output _newgun_2)
    (`/Game/Blueprints/FPSChar_V_0_3.BuildWeapon` _newparam))
  (`self.K2_DestroyActor`))

(fn `Add Blood on Crit`
  (params (Gun :type "/Game/FirstPersonBP/Blueprints/Guns/GunVariables Structure") (BloodOnCrit :type "Float (double-precision)"))
  (returns (NewGun :type "/Game/FirstPersonBP/Blueprints/Guns/GunVariables Structure"))
  (return))

(fn `Ammo on Crit`
  (params (Gun :type "/Game/FirstPersonBP/Blueprints/Guns/GunVariables Structure") (AddAmmoOnCrit :type "Float (double-precision)"))
  (returns (NewGun :type "/Game/FirstPersonBP/Blueprints/Guns/GunVariables Structure"))
  (return))

(fn `UserConstructionScript`
  (`parent.UserConstructionScript`))