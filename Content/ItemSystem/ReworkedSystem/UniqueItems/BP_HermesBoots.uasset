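; Hermes Boots is a unique item pickup that raises the player's maximum number of dash charges.
; On interact, it runs the parent item logic, adds its AddedDashCharges value to the player's DashMaxCharges through a small helper function, then destroys itself.
; The bonus goes to the actor returned by GetPlayer, and only the maximum is changed directly.
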(event `/Game/Inventory/Interact_Interface.ItemInteract`
  (params (Interactor :type "Actor Object Reference"))
  (`parent.ItemInteract` Interactor)
  (bind _newparam (`self.GetPlayer`))
  (bind _newdashcharges (`self.NewFunction_0` (`/Game/Blueprints/FPSChar_V_0_3.DashMaxCharges` _newparam) (`self.AddedDashCharges`)))
  (set `/Game/Blueprints/FPSChar_V_0_3.DashMaxCharges` _newdashcharges _newparam)
  (`self.K2_DestroyActor`))

(fn `NewFunction_0`
  (params (DashCharges :type Integer) (AddedDashCharges :type Integer))
  (returns (NewDashCharges :type Integer))
  (return (+ DashCharges AddedDashCharges)))

(fn `UserConstructionScript`
  (`parent.UserConstructionScript`))