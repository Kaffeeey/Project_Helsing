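; Scorched Angel Wings is a unique item pickup that grants the player extra jumps.
; On interact it runs the parent item logic, then uses ChangeJumpCount to add AddJumpCount to the player's JumpMaxCount and destroys itself.
; The bonus is applied to the character returned by GetPlayer rather than to the Interactor passed into the event.
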(event `/Game/Inventory/Interact_Interface.ItemInteract`
  (params (Interactor :type "Actor Object Reference"))
  (`parent.ItemInteract` Interactor)
  (bind _newparam (`self.GetPlayer`))
  (bind _newjumpamount (`self.ChangeJumpCount` (`Character.JumpMaxCount` _newparam) (`self.AddJumpCount`)))
  (set `Character.JumpMaxCount` _newjumpamount _newparam)
  (`self.K2_DestroyActor`))

(fn `ChangeJumpCount`
  (params (CurrentJumpAmount :type Integer) (AddedJumpAmount :type Integer))
  (returns (NewJumpAmount :type Integer))
  (return (+ CurrentJumpAmount AddedJumpAmount)))

(fn `UserConstructionScript`
  (`parent.UserConstructionScript`))