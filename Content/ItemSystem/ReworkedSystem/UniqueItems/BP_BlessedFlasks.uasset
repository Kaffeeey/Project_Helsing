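; Blessed Flasks unique item that permanently expands the player's potion capacity when interacted with.
; After the parent interact logic, it adds AddFlaskLimit to the player's FullPotionMaxAmount through a small helper function.
; It reveals hard-wired HUD slots Potion6 to Potion8 with their inner Potion2 element hidden and appends them to PotionArray, regardless of the limit value.
; The actor then destroys itself.
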(event `/Game/Inventory/Interact_Interface.ItemInteract`
  (params (Interactor :type "Actor Object Reference"))
  (`parent.ItemInteract` Interactor)
  (bind _newparam (`self.GetPlayer`))
  (bind _newpotionlimit (`self.Add Potion Limit` (`/Game/Blueprints/FPSChar_V_0_3.FullPotionMaxAmount` _newparam) (`self.AddFlaskLimit`)))
  (set `/Game/Blueprints/FPSChar_V_0_3.FullPotionMaxAmount` _newpotionlimit _newparam)
  (bind _hud (`/Game/Blueprints/FPSChar_V_0_3.HUD` _newparam))
  (bind _potion6 (`/Game/HUD_TEST/Widget_HUD.Potion6` _hud))
  (`Widget.SetVisibility` _potion6 "Visible")
  (`Widget.SetVisibility` (`/Game/HUD_TEST/Potion.Potion2` _potion6) "Hidden")
  (bind _potionarray (`/Game/HUD_TEST/Widget_HUD.PotionArray` _hud))
  (`KismetArrayLibrary.Array_Add` _potionarray _potion6)
  (bind _potion7 (`/Game/HUD_TEST/Widget_HUD.Potion7` _hud))
  (`Widget.SetVisibility` _potion7 "Visible")
  (`Widget.SetVisibility` (`/Game/HUD_TEST/Potion.Potion2` _potion7) "Hidden")
  (`KismetArrayLibrary.Array_Add` _potionarray _potion7)
  (bind _potion8 (`/Game/HUD_TEST/Widget_HUD.Potion8` _hud))
  (`Widget.SetVisibility` _potion8 "Visible")
  (`Widget.SetVisibility` (`/Game/HUD_TEST/Potion.Potion2` _potion8) "Hidden")
  (`KismetArrayLibrary.Array_Add` _potionarray _potion8)
  (`self.K2_DestroyActor`))

(fn `Add Potion Limit`
  (params (CurrentPotionLimit :type Integer) (AddPotionLimit :type Integer))
  (returns (NewPotionLimit :type Integer))
  (return (+ CurrentPotionLimit AddPotionLimit)))

(fn `UserConstructionScript`
  (`parent.UserConstructionScript`))