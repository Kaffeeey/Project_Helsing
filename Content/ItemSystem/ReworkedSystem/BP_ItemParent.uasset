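; BP_ItemParent is the base Blueprint for interactable items that remove their matching copies from the level.
; ItemInteract scans all BP_ItemParent actors and destroys those matching its UniqueItem when IsUnique, or its StageItem otherwise, then destroys itself.
; A GetPlayer helper looks up the FPSChar_V_0_3 character by class; construction, BeginPlay, overlap and Tick are empty.
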(event `/Game/Inventory/Interact_Interface.ItemInteract`
  (params (Interactor :type "Actor Object Reference"))
  (bind _outactors (`GameplayStatics.GetAllActorsOfClass` "BP_ItemParent_C"))
  (for _array_element _outactors
    (if (`self.IsUnique`)
      (if (`|EnumEquality` (`self.UniqueItem`) (`/Game/ItemSystem/ReworkedSystem/BP_ItemParent.UniqueItem` _array_element))
        (`self.K2_DestroyActor` _array_element))
      (elif (`|EnumEquality` (`/Game/ItemSystem/ReworkedSystem/BP_ItemParent.StageItem` _array_element) (`self.StageItem`))
        (`self.K2_DestroyActor` _array_element))))
  (`self.K2_DestroyActor`))

(fn `GetPlayer`
  (returns (NewParam :type "/Game/Blueprints/FPSChar_V_0_3 Object Reference"))
  (bind _returnvalue (`GameplayStatics.GetActorOfClass` "/Game/Blueprints/FPSChar_V_0_3.FPSChar_V_0_3_C"))
  (return _returnvalue))

(fn `UserConstructionScript`)