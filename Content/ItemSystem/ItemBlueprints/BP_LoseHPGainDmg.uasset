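; Interactable item pickup that, as its name indicates, trades player max HP for gun damage, then destroys itself.
; On interact, it loops over three gun slots, saving the current gun, adding to that slot's DamageAmp through a copied struct, and rebuilding the weapon.
; It then offsets MaxHP, also setting HP to the new maximum unless HP already exceeds it, so excess HP is left unclamped.
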(event `/Game/Inventory/Interact_Interface.Interact`
  (params (Interactor :type "Actor Object Reference"))
  (`parent.Interact` Interactor)
  (bind _player (`self.GetPlayer`))
  (for _index (range 3)
    (`/Game/Blueprints/FPSChar_V_0_3.SaveCurrentGun` _player)
    (bind _output (`|GetArrayItem` (`/Game/Blueprints/FPSChar_V_0_3.GunArray` _player) _index))
    (bind _newgun (`self.Change Percent Damage` _output (`self.ChangePercentDamage`)))
    (`|VariableSetRef` _output _newgun)
    (`/Game/Blueprints/FPSChar_V_0_3.BuildWeapon` _player))
  (bind _newhealth (`self.Change Max Health` (`self.ChangeMaxHealth`) (`/Game/Blueprints/FPSChar_V_0_3.MaxHP` _player)))
  (if (> (`/Game/Blueprints/FPSChar_V_0_3.HP` _player) _newhealth)
    (set `/Game/Blueprints/FPSChar_V_0_3.MaxHP` _newhealth _player)
    (else
      (bind _output_get (set `/Game/Blueprints/FPSChar_V_0_3.HP` _newhealth _player))
      (set `/Game/Blueprints/FPSChar_V_0_3.MaxHP` _output_get _player)))
  (`self.K2_DestroyActor`))

(fn `Change Max Health`
  (params (AddHealth :type "Float (double-precision)") (CurrentMaxHealth :type "Float (double-precision)"))
  (returns (NewHealth :type "Float (double-precision)"))
  (return (+ AddHealth CurrentMaxHealth)))

(fn `Change Percent Damage`
  (params (OldGun :type "/Game/FirstPersonBP/Blueprints/Guns/GunVariables Structure") (AddPercentDamage :type "Float (double-precision)"))
  (returns (NewGun :type "/Game/FirstPersonBP/Blueprints/Guns/GunVariables Structure"))
  (return (make `/Game/FirstPersonBP/Blueprints/Guns/GunVariables` OldGun_GunType_2_14FC35544E58478CA236669C8A25613F OldGun_AmmoCurrent_5_5302FF684AA84A1D4269D996DDF371EA OldGun_AmmoMax_7_5F39C5A345B67AEE2D137699778EDCFD OldGun_BulletAngle_13_BFD283954948BD292AA064BFA0F8E516 OldGun_Damage_17_99EB532E4ED9FC782950138E04B2F512 OldGun_ClipSize_20_3B0274BE43EBE86114EAD6A682365631 (+ AddPercentDamage OldGun_DamageAmp_25_734A8F6241C66E18F8506C9CDF54D76E) OldGun_ClipCount_28_66C030C441DA950025982B936A504732 OldGun_Bullets_32_94AD3E4E46EB673342C43EB25F42E653 OldGun_BoltType_36_F8ADBC2D4954BBB8298E108193B2078D OldGun_MaxAmmoLimit_39_E9180C084BC0FD87DC0099BE96B5F6C7 OldGun_KnockbackStrengthMultiplier_43_5DF9E7DC44733A2B82F379BAACE4A378 OldGun_ReloadTimeReduction_46_764E97C24ED54D09720A80BF7A086918 OldGun_ReloadOnSwap_49_5273A4EB49D327EAD27B7EA53FFEB553 OldGun_CritMultiplier_54_FD153910476009D858F2EF8FA7CD60ED OldGun_PiercingBullets_52_F919B5B7494EBC48894AEAB37D83D932 OldGun_CritChance_57_6C7773F1480E01B5C401CC94A9B11E98 OldGun_AmmoOnCrit_83_DF1B68634193D27A4D5473BC552235F8 OldGun_GoldenChance_63_F512CEC843A90B444CA310AC5EF4EE5E OldGun_ReloadWeaponOnHit_68_3498DF844B1A89273EC82BA630D9EB01 OldGun_StunOnHit_69_23E8D78D4D5712661930D58EEECD3E84 OldGun_BloodOnCrit_82_5A55CE534D8E6E07EF7B7BBB2E920952 OldGun_NearbyDamageOnCrit_81_2DEDA9ED4855CBC0A820DFA7292A1EA3 OldGun_LastBulletDamage_80_1D69B9EE4F228D3E5AE782A956DCA5D6 OldGun_CashOnCrit_89_501F8B734C5439FC0B98DDBD6FB96B72 OldGun_BloodOnArealKill_91_4088028046EF146BAA56FC93122D04C3 OldGun_HealOnEnemyKill_94_13C4736D47C3BF73488A1B87D406C2E1 OldGun_ReduceCDsOnKill_96_18AAEC864D5AFDF9092A6F839BDFEC25)))

(fn `UserConstructionScript`
  (`parent.UserConstructionScript`))