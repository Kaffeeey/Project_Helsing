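; Interactable item that permanently changes the player's hook range, then removes itself from the world.
; On ItemInteract it runs the parent logic, then adds its AddHookRange value to the HookRange of the player returned by GetPlayer, not the passed Interactor.
; A small helper function performs the sum, and the actor destroys itself after writing the new range back to the player.
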(event `/Game/Inventory/Interact_Interface.ItemInteract`
  (params (Interactor :type "Actor Object Reference"))
  (`parent.ItemInteract` Interactor)
  (bind _player (`self.GetPlayer`))
  (bind _newhookrange (`self.Add Hook Range` (`self.AddHookRange`) (`/Game/Blueprints/FPSChar_V_0_3.HookRange` _player)))
  (set `/Game/Blueprints/FPSChar_V_0_3.HookRange` _newhookrange _player)
  (`self.K2_DestroyActor`))

(fn `Add Hook Range`
  (params (CurrentHookRange :type "Float (double-precision)") (AddHookRange :type "Float (double-precision)"))
  (returns (NewHookRange :type "Float (double-precision)"))
  (return (+ CurrentHookRange AddHookRange)))

(fn `UserConstructionScript`
  (`parent.UserConstructionScript`))