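; BP_ParentTickItem is an interactable item, named as a parent class, for temporary player buffs.
; On interact, it clears and destroys same-class entries in the character's TempBuffs to prevent stacking, then registers itself there.
; ApplyBuff and ClearBuff raise and lower MaxHP by a fixed amount.
; The chain that applies the buff, removes pickup components and expires after BuffDuration is unconnected, so this graph never applies it.
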(event `/Game/Inventory/Interact_Interface.Interact`
  (params (Interactor :type "Actor Object Reference"))
  (`parent.Interact` Interactor)
  (bind _asfpschar_v_0_3 (cast `/Game/Blueprints/FPSChar_V_0_3` Interactor))
  (`self.CheckForDuplicates` Interactor)
  (`KismetArrayLibrary.Array_Add` (`/Game/Blueprints/FPSChar_V_0_3.TempBuffs` _asfpschar_v_0_3) self))

(fn `ApplyBuff`
  (params (NewParam :type "Actor Object Reference"))
  (bind _asfpschar_v_0_3 (cast `/Game/Blueprints/FPSChar_V_0_3` NewParam))
  (set `/Game/Blueprints/FPSChar_V_0_3.MaxHP` (+ (`/Game/Blueprints/FPSChar_V_0_3.MaxHP` _asfpschar_v_0_3) 5.0) _asfpschar_v_0_3))

(fn `CheckForDuplicates`
  (params (NewParam :type "Actor Object Reference"))
  (bind _asfpschar_v_0_3 (cast `/Game/Blueprints/FPSChar_V_0_3` NewParam))
  (for _array_element (`/Game/Blueprints/FPSChar_V_0_3.TempBuffs` _asfpschar_v_0_3)
    (`/Engine/EditorBlueprintResources/StandardMacros.IsValid` _array_element
      (:`Is Valid`
        (if (== (`GameplayStatics.GetObjectClass` _array_element) (`GameplayStatics.GetObjectClass` self))
          (bind _asbp_parent_tick_item (cast `/Game/ItemSystem/ItemBlueprints/BP_ParentTickItem` _array_element))
          (`self.ClearBuff` _asbp_parent_tick_item _asfpschar_v_0_3)
          (`self.K2_DestroyActor` _array_element))))))

(fn `ClearBuff`
  (params (NewParam :type "Actor Object Reference"))
  (bind _asfpschar_v_0_3 (cast `/Game/Blueprints/FPSChar_V_0_3` NewParam))
  (set `/Game/Blueprints/FPSChar_V_0_3.MaxHP` (- (`/Game/Blueprints/FPSChar_V_0_3.MaxHP` _asfpschar_v_0_3) 5.0) _asfpschar_v_0_3))

(fn `UserConstructionScript`
  (`parent.UserConstructionScript`))