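; BP_ChangeSpeed is an interactable item that changes the player's walk speed and is consumed on use.
; On ItemInteract it runs the parent logic, then passes the player's current MaxWalkSpeed and the item's AddSpeed to ChangeSpeed.
; ChangeSpeed adds the two and caps the sum at SpeedLimit; the result is written back to CharacterMovement before the actor destroys itself.
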(event `/Game/Inventory/Interact_Interface.ItemInteract`
  (params (Interactor :type "Actor Object Reference"))
  (`parent.ItemInteract` Interactor)
  (bind _player (`self.GetPlayer`))
  (bind _charactermovement (`Character.CharacterMovement` _player))
  (bind _newspeed (`self.Change Speed` (`self.AddSpeed`) (`CharacterMovementComponent.MaxWalkSpeed` _charactermovement)))
  (set `CharacterMovementComponent.MaxWalkSpeed` _newspeed _charactermovement)
  (`self.K2_DestroyActor`))

(fn `Change Speed`
  (params (AddSpeed :type "Float (double-precision)") (CurrentSpeed :type "Float (double-precision)"))
  (returns (NewSpeed :type "Float (double-precision)"))
  (return (`KismetMathLibrary.FMin` (+ AddSpeed CurrentSpeed) (`self.SpeedLimit`))))

(fn `UserConstructionScript`
  (`parent.UserConstructionScript`))