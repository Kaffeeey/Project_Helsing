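; An interactable item that raises the player's DoubleEffectForFlask stat, then removes itself from the world.
; On ItemInteract it runs the parent logic, then passes the player's current value and its own AddedFlaskDuality amount to the FlaskDuality function.
; That function returns their sum, which is written back to the player before the actor is destroyed.
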(event `/Game/Inventory/Interact_Interface.ItemInteract`
  (params (Interactor :type "Actor Object Reference"))
  (`parent.ItemInteract` Interactor)
  (bind _player (`self.GetPlayer`))
  (bind _newflaskduality (`self.Flask Duality` (`/Game/Blueprints/FPSChar_V_0_3.DoubleEffectForFlask` _player) (`self.AddedFlaskDuality`)))
  (set `/Game/Blueprints/FPSChar_V_0_3.DoubleEffectForFlask` _newflaskduality _player)
  (`self.K2_DestroyActor`))

(fn `Flask Duality`
  (params (FlaskDuality :type "Float (double-precision)") (AddFlaskDuality :type "Float (double-precision)"))
  (returns (NewFlaskDuality :type "Float (double-precision)"))
  (return (+ FlaskDuality AddFlaskDuality)))

(fn `UserConstructionScript`
  (`parent.UserConstructionScript`))