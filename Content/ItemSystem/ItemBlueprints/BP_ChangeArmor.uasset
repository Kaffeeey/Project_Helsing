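; Interactable item Blueprint that changes the player's armor when used, then removes itself from the world.
; ItemInteract calls the parent handler, fetches the player through GetPlayer rather than the Interactor, and writes back a new Armor value.
; The ChangeArmor helper simply adds the item's AddArmor amount to current Armor, with no clamping.
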(event `/Game/Inventory/Interact_Interface.ItemInteract`
  (params (Interactor :type "Actor Object Reference"))
  (`parent.ItemInteract` Interactor)
  (bind _player (`self.GetPlayer`))
  (bind _newarmor (`self.Change Armor` (`/Game/Blueprints/FPSChar_V_0_3.Armor` _player) (`self.AddArmor`)))
  (set `/Game/Blueprints/FPSChar_V_0_3.Armor` _newarmor _player)
  (`self.K2_DestroyActor`))

(fn `Change Armor`
  (params (Armor :type "Float (double-precision)") (ArmorerChange :type "Float (double-precision)"))
  (returns (NewArmor :type "Float (double-precision)"))
  (return (+ Armor ArmorerChange)))

(fn `UserConstructionScript`
  (`parent.UserConstructionScript`))