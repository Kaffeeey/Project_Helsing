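; BP_ChangeJumpCount is an interactable item that changes how many jumps the player can make.
; On ItemInteract it runs the parent logic, then uses ChangeJumpCount to add JumpAmountAdded to the player's JumpMaxCount.
; The target comes from GetPlayer rather than the Interactor argument, and the item destroys itself afterwards.
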(event `/Game/Inventory/Interact_Interface.ItemInteract`
  (params (Interactor :type "Actor Object Reference"))
  (`parent.ItemInteract` Interactor)
  (bind _player (`self.GetPlayer`))
  (bind _newjumpamount (`self.ChangeJumpCount` (`Character.JumpMaxCount` _player) (`self.JumpAmountAdded`)))
  (set `Character.JumpMaxCount` _newjumpamount _player)
  (`self.K2_DestroyActor`))

(fn `ChangeJumpCount`
  (params (CurrentJumpAmount :type Integer) (AddedJumpAmount :type Integer))
  (returns (NewJumpAmount :type Integer))
  (return (+ CurrentJumpAmount AddedJumpAmount)))

(fn `UserConstructionScript`
  (`parent.UserConstructionScript`))