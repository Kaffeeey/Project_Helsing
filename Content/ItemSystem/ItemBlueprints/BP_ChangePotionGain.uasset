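; BP_ChangePotionGain is an interactable item that adjusts the player's PotionGain stat when used.
; On ItemInteract it runs the parent logic, then adds its AddPotionGain value to the current PotionGain through the ChangePotionGain helper function.
; It writes the sum back to the player returned by GetPlayer, regardless of the Interactor, and destroys itself, making it a one-time pickup.
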(event `/Game/Inventory/Interact_Interface.ItemInteract`
  (params (Interactor :type "Actor Object Reference"))
  (`parent.ItemInteract` Interactor)
  (bind _player (`self.GetPlayer`))
  (bind _newpotiongain (`self.Change Potion Gain` (`/Game/Blueprints/FPSChar_V_0_3.PotionGain` _player) (`self.AddPotionGain`)))
  (set `/Game/Blueprints/FPSChar_V_0_3.PotionGain` _newpotiongain _player)
  (`self.K2_DestroyActor`))

(fn `Change Potion Gain`
  (params (CurrentPotionGain :type "Float (double-precision)") (AddedPotionGain :type "Float (double-precision)"))
  (returns (NewPotionGain :type "Float (double-precision)"))
  (return (+ CurrentPotionGain AddedPotionGain)))

(fn `UserConstructionScript`
  (`parent.UserConstructionScript`))