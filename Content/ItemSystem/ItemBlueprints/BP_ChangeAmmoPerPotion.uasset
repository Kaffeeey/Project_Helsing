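; BP_ChangeAmmoPerPotion is an interactable item that raises how much ammo the player gains per potion.
; On ItemInteract it runs the parent logic, then fetches the player and adds AddedAmmoPerPotion to the player's AmmoGain through a small addition function.
; It then destroys itself, so each pickup applies once.
; The interactor is only passed to the parent; the bonus always goes to the GetPlayer result.
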(event `/Game/Inventory/Interact_Interface.ItemInteract`
  (params (Interactor :type "Actor Object Reference"))
  (`parent.ItemInteract` Interactor)
  (bind _player (`self.GetPlayer`))
  (bind _newammoperpotion (`self.Add Ammo Per Potion` (`/Game/Blueprints/FPSChar_V_0_3.AmmoGain` _player) (`self.AddedAmmoPerPotion`)))
  (set `/Game/Blueprints/FPSChar_V_0_3.AmmoGain` _newammoperpotion _player)
  (`self.K2_DestroyActor`))

(fn `Add Ammo Per Potion`
  (params (CurrentAmmoPerPotion :type Integer) (AddAmmoPerPotion :type Integer))
  (returns (NewAmmoPerPotion :type Integer))
  (return (+ CurrentAmmoPerPotion AddAmmoPerPotion)))

(fn `UserConstructionScript`
  (`parent.UserConstructionScript`))