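; Item Blueprint that changes the player's dash range when interacted with, then removes itself.
; On ItemInteract it runs the parent logic, gets the player and passes its DashRange with the item's AddDashRange value through a simple addition function.
; The sum is written back to the player's DashRange before the actor is destroyed.
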(event `/Game/Inventory/Interact_Interface.ItemInteract`
  (params (Interactor :type "Actor Object Reference"))
  (`parent.ItemInteract` Interactor)
  (bind _player (`self.GetPlayer`))
  (bind _newdashrange (`self.Add Dash Range` (`/Game/Blueprints/FPSChar_V_0_3.DashRange` _player) (`self.AddDashRange`)))
  (set `/Game/Blueprints/FPSChar_V_0_3.DashRange` _newdashrange _player)
  (`self.K2_DestroyActor`))

(fn `Add Dash Range`
  (params (CurrentDashRange :type "Float (double-precision)") (AddDashRange :type "Float (double-precision)"))
  (returns (NewDashRange :type "Float (double-precision)"))
  (return (+ CurrentDashRange AddDashRange)))

(fn `UserConstructionScript`
  (`parent.UserConstructionScript`))