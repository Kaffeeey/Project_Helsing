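; BP_ChangeAmmoAndHPPerPotion is an interactable item that permanently raises how much HP and ammo the player gains per potion.
; On Interact, it calls the parent logic, then adds its AddHPPerPotion and AddAmmoPerPotion amounts to the player's HPGain and AmmoGain through two simple addition functions.
; It then destroys itself, making it a one-time pickup.
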(event `/Game/Inventory/Interact_Interface.Interact`
  (params (Interactor :type "Actor Object Reference"))
  (`parent.Interact` Interactor)
  (bind _player (`self.GetPlayer`))
  (bind _newhp_perpotion (`self.HP Per Potion` (`/Game/Blueprints/FPSChar_V_0_3.HPGain` _player) (`self.AddHPPerPotion`)))
  (set `/Game/Blueprints/FPSChar_V_0_3.HPGain` _newhp_perpotion _player)
  (bind _newammoperpotion (`self.Add Ammo Per Potion` (`/Game/Blueprints/FPSChar_V_0_3.AmmoGain` _player) (`self.AddAmmoPerPotion`)))
  (set `/Game/Blueprints/FPSChar_V_0_3.AmmoGain` _newammoperpotion _player)
  (`self.K2_DestroyActor`))

(fn `Add Ammo Per Potion`
  (params (CurrentAmmoPerPotion :type Integer) (AddAmmoPerPotion :type Integer))
  (returns (NewAmmoPerPotion :type Integer))
  (return (+ CurrentAmmoPerPotion AddAmmoPerPotion)))

(fn `HP Per Potion`
  (params (`CurrentHP PerPotion` :type "Float (double-precision)") (`AddedHP PerPotion` :type "Float (double-precision)"))
  (returns (`NewHP PerPotion` :type "Float (double-precision)"))
  (return (+ `CurrentHP PerPotion` `AddedHP PerPotion`)))

(fn `UserConstructionScript`
  (`parent.UserConstructionScript`))