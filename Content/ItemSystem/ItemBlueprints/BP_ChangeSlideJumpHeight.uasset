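; BP_ChangeSlideJumpHeight is an interactable item meant to change the player's slide jump height.
; On interaction it calls the parent logic, passes the player's current height and AddSlideJumpHeight to ChengeSlideJumpHeight, writes the result back, then destroys itself.
; The helper ignores both inputs and returns zero as written, so the interaction sets the player's slide jump height to zero.
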(event `/Game/Inventory/Interact_Interface.ItemInteract`
  (params (Interactor :type "Actor Object Reference"))
  (`parent.ItemInteract` Interactor)
  (bind _player (`self.GetPlayer`))
  (bind _newslidejumpheight (`self.Chenge Slide Jump Height` (`/Game/Blueprints/FPSChar_V_0_3.SlideJumpheight` _player) (`self.AddSlideJumpHeight`)))
  (set `/Game/Blueprints/FPSChar_V_0_3.SlideJumpheight` _newslidejumpheight _player)
  (`self.K2_DestroyActor`))

(fn `Chenge Slide Jump Height`
  (params (CurrentSlideJumpHeight :type "Float (double-precision)") (AddedSlideJumpHeight :type "Float (double-precision)"))
  (returns (NewSlideJumpHeight :type "Float (double-precision)"))
  (return 0.0))

(fn `UserConstructionScript`
  (`parent.UserConstructionScript`))