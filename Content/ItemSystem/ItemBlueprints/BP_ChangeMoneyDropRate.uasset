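; BP_ChangeMoneyDropRate is an interactable item that modifies the player's money drop chance.
; On Interact it runs the parent logic, adds its configured ChangeMoneyDroptRate amount to the player's MoneyDropChance through a simple addition function, then destroys itself.
; The change is a plain additive write to the player variable, with no clamping or timed revert in this Blueprint.
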(event `/Game/Inventory/Interact_Interface.Interact`
  (params (Interactor :type "Actor Object Reference"))
  (`parent.Interact` Interactor)
  (bind _player (`self.GetPlayer`))
  (bind _newmoneydroprate (`self.Change Money Drop Rate` (`/Game/Blueprints/FPSChar_V_0_3.MoneyDropChance` _player) (`self.ChangeMoneyDroptRate`)))
  (set `/Game/Blueprints/FPSChar_V_0_3.MoneyDropChance` _newmoneydroprate _player)
  (`self.K2_DestroyActor`))

(fn `Change Money Drop Rate`
  (params (CurrentMoneyDropRate :type "Float (double-precision)") (AddMoneyDropRate :type "Float (double-precision)"))
  (returns (NewMoneyDropRate :type "Float (double-precision)"))
  (return (+ CurrentMoneyDropRate AddMoneyDropRate)))

(fn `UserConstructionScript`
  (`parent.UserConstructionScript`))