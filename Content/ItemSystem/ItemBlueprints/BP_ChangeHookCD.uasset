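; BP_ChangeHookCD is an interactable item that changes the player's hook cooldown when used, then destroys itself.
; On ItemInteract it runs the parent logic, then gets the player and passes HookCooldownReduktion and the item's ReduceHookCD value to a helper function.
; The helper sums both values, and the result is written to HookCooldown rather than back to HookCooldownReduktion.
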(event `/Game/Inventory/Interact_Interface.ItemInteract`
  (params (Interactor :type "Actor Object Reference"))
  (`parent.ItemInteract` Interactor)
  (bind _player (`self.GetPlayer`))
  (bind _newhookcd (`self.Reduce Hook CD` (`/Game/Blueprints/FPSChar_V_0_3.HookCooldownReduktion` _player) (`self.ReduceHookCD`)))
  (set `/Game/Blueprints/FPSChar_V_0_3.HookCooldown` _newhookcd _player)
  (`self.K2_DestroyActor`))

(fn `Reduce Hook CD`
  (params (CurrentHookCD :type "Float (double-precision)") (AddHookCD :type "Float (double-precision)"))
  (returns (NewHookCD :type "Float (double-precision)"))
  (return (+ CurrentHookCD AddHookCD)))

(fn `UserConstructionScript`
  (`parent.UserConstructionScript`))