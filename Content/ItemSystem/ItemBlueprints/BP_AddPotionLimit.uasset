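; BP_AddPotionLimit is an interactable item that raises the player's maximum potion capacity.
; On Interact it runs the parent behavior, then adds its AddPotionLimit value to the player's FullPotionMaxAmount through a simple addition function.
; It changes the player returned by GetPlayer rather than using the Interactor directly, then destroys itself as a one-time pickup.
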(event `/Game/Inventory/Interact_Interface.Interact`
  (params (Interactor :type "Actor Object Reference"))
  (`parent.Interact` Interactor)
  (bind _player (`self.GetPlayer`))
  (bind _newpotionlimit (`self.Add Potion Limit` (`/Game/Blueprints/FPSChar_V_0_3.FullPotionMaxAmount` _player) (`self.AddPotionLimit`)))
  (set `/Game/Blueprints/FPSChar_V_0_3.FullPotionMaxAmount` _newpotionlimit _player)
  (`self.K2_DestroyActor`))

(fn `Add Potion Limit`
  (params (CurrentPotionLimit :type Integer) (AddPotionLimit :type Integer))
  (returns (NewPotionLimit :type Integer))
  (return (+ CurrentPotionLimit AddPotionLimit)))

(fn `UserConstructionScript`
  (`parent.UserConstructionScript`))