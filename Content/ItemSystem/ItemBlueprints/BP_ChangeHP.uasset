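; BP_ChangeHP is an interactable item that changes the player's maximum health.
; On Interact it runs the parent logic, gets the player, and sets MaxHP to the current value plus the item's AddMaxHP amount.
; The sum comes from a small ChangeMaxHealth helper function, and the actor destroys itself afterwards, making it single-use.
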(event `/Game/Inventory/Interact_Interface.Interact`
  (params (Interactor :type "Actor Object Reference"))
  (`parent.Interact` Interactor)
  (bind _player (`self.GetPlayer`))
  (bind _newhealth (`self.Change Max Health` (`self.AddMaxHP`) (`/Game/Blueprints/FPSChar_V_0_3.MaxHP` _player)))
  (set `/Game/Blueprints/FPSChar_V_0_3.MaxHP` _newhealth _player)
  (`self.K2_DestroyActor`))

(fn `Change Max Health`
  (params (AddHealth :type "Float (double-precision)") (CurrentMaxHealth :type "Float (double-precision)"))
  (returns (NewHealth :type "Float (double-precision)"))
  (return (+ AddHealth CurrentMaxHealth)))

(fn `UserConstructionScript`
  (`parent.UserConstructionScript`))