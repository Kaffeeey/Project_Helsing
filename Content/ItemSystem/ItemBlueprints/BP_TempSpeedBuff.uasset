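; BP_TempSpeedBuff is an item that, when interacted with, raises the FPSChar_V_0_3 interactor's MovementSpeed by SpeedChange.
; It calls the parent Interact, destroys its root, mesh, shell and rarity effect components, then waits BuffDuration before destroying itself.
; After the delay it writes MovementSpeed minus SpeedChange into MaxHP instead of MovementSpeed, so the speed boost is never reverted and MaxHP is overwritten.
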(event `/Game/Inventory/Interact_Interface.Interact`
  (params (Interactor :type "Actor Object Reference"))
  (`parent.Interact` Interactor)
  (bind _asfpschar_v_0_3 (cast `/Game/Blueprints/FPSChar_V_0_3` Interactor))
  (set `/Game/Blueprints/FPSChar_V_0_3.MovementSpeed` (+ (`/Game/Blueprints/FPSChar_V_0_3.MovementSpeed` _asfpschar_v_0_3) (`self.SpeedChange`)) _asfpschar_v_0_3)
  (`ActorComponent.K2_DestroyComponent` (`self.DefaultSceneRoot`))
  (`ActorComponent.K2_DestroyComponent` (`self.Shell`))
  (`ActorComponent.K2_DestroyComponent` (`self.StaticMesh`))
  (`ActorComponent.K2_DestroyComponent` (`self.NS_ItemRarity`))
  (`KismetSystemLibrary.Delay` (`self.BuffDuration`))
  (set `/Game/Blueprints/FPSChar_V_0_3.MaxHP` (- (`/Game/Blueprints/FPSChar_V_0_3.MovementSpeed` _asfpschar_v_0_3) (`self.SpeedChange`)) _asfpschar_v_0_3)
  (`self.K2_DestroyActor`))

(fn `UserConstructionScript`
  (`parent.UserConstructionScript`))