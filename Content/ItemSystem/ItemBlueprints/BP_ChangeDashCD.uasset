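; BP_ChangeDashCD is an interactable item that changes the player's dash cooldown and then destroys itself.
; On Interact it runs the parent logic, then adds its ReduceDashCD amount to the player's DashCooldownReduction through a simple addition function.
; The sum is written to the player's DashCooldown rather than back to DashCooldownReduction.
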(event `/Game/Inventory/Interact_Interface.Interact`
  (params (Interactor :type "Actor Object Reference"))
  (`parent.Interact` Interactor)
  (bind _player (`self.GetPlayer`))
  (bind _newdashcd (`self.Reduce Dash CD` (`/Game/Blueprints/FPSChar_V_0_3.DashCooldownReduction` _player) (`self.ReduceDashCD`)))
  (set `/Game/Blueprints/FPSChar_V_0_3.DashCooldown` _newdashcd _player)
  (`self.K2_DestroyActor`))

(fn `Reduce Dash CD`
  (params (CurrentDashCD :type "Float (double-precision)") (AddDashCD :type "Float (double-precision)"))
  (returns (NewDashCD :type "Float (double-precision)"))
  (return (+ CurrentDashCD AddDashCD)))

(fn `UserConstructionScript`
  (`parent.UserConstructionScript`))