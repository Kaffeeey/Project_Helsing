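; BP_TextTrigger is a tutorial trigger that shows a "Press {key} to {action}" prompt when FPSChar_V_0_3 overlaps it.
; It looks up the keys mapped to ActionName and writes the key name and ActionDescription into the character's TutorialText widget.
; Both loop body and completion feed the same text update, so the last mapping's key remains displayed.
; After UpDuration it hides the widget and destroys itself, making the prompt one-shot.
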(event `self.ReceiveActorBeginOverlap`
  (params (OtherActor :type "Actor Object Reference"))
  (bind _asfpschar_v_0_3 (cast `/Game/Blueprints/FPSChar_V_0_3` OtherActor))
  (for _array_element (`InputSettings.GetActionMappingByName` (`InputSettings.GetInputSettings`) (`self.ActionName`))
    (bind _tutorialtext (`/Game/HUD_TEST/Widget_TutorialText2.TutorialText` (`/Game/Blueprints/FPSChar_V_0_3.Tutorial` _asfpschar_v_0_3)))
    (`TextBlock.SetText` (`/Game/HUD_TEST/TutorialText.TextBlock_0` _tutorialtext) (`|FormatText` "Press {0} to {1}" (`KismetInputLibrary.Key_GetDisplayName` (`.Key` (break `InputActionKeyMapping` _array_element))) (`self.ActionDescription`)) :!label _label)
    (`Widget.SetVisibility` _tutorialtext "Visible")
    (`KismetSystemLibrary.Delay` (`self.UpDuration`))
    (`Widget.SetVisibility` _tutorialtext "Hidden")
    (`self.K2_DestroyActor`))
  (goto _label))

(fn `UserConstructionScript`)