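; Enemy actor that fires Wurm_Projectile_BP projectiles, takes damage and destroys itself when HP drops to zero or below.
; StartShooting makes one FireBullet attempt, spawning at BulletPoint with the capsule's rotation, while StopShooting is empty.
; Each shot resets a timer that Tick advances up to FireRate, the cooldown before CanFire returns.
; GetDamage sets HP to Damage minus HP, an apparently reversed subtraction.
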(event `self.ReceiveBeginPlay`
  (set `self.MomFireRate` (`self.FireRate`))
  (set `self.CanFire` true))

(event `StartShooting`
  (`self.FireBullet`))

(event `StopShooting`)

(event `self.ReceiveTick`
  (params (DeltaSeconds :type "Float (single-precision)"))
  (if (< (`self.MomFireRate`) (`self.FireRate`))
    (set `self.MomFireRate` (+ (`self.MomFireRate`) (`GameplayStatics.GetWorldDeltaSeconds`)))
    (if (>= (`self.MomFireRate`) (`self.FireRate`))
      (set `self.MomFireRate` (`self.FireRate`))
      (set `self.CanFire` true))))

(fn `FireBullet`
  (if (`self.CanFire`)
    (`|SpawnActorFromClass` "/Game/Blueprints/Wurm_Projectile_BP.Wurm_Projectile_BP_C" (`KismetMathLibrary.MakeTransform` (`SceneComponent.K2_GetComponentLocation` (`self.BulletPoint`)) (`SceneComponent.GetSocketRotation` (`self.CapsuleComponent`) "None")) "Undefined" "OverrideRootScale" null null)
    (set `self.CanFire` false)
    (set `self.MomFireRate` 0.0)))

(fn `GetDamage`
  (params (Damage :type "Float (double-precision)"))
  (set `self.HP` (- Damage (`self.HP`)))
  (if (<= (`self.HP`) 0.0)
    (`self.K2_DestroyActor`)))

(fn `UserConstructionScript`)