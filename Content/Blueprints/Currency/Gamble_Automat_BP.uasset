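; Gambling machine actor that, on Interact, sells the player a random chance at an item for Currency, up to a maximum number of plays.
; Each paid play multiplies the price, then rolls against the current item chance.
; A win spawns the item in front of the machine and resets the chance, while a loss raises it for the next play as a pity mechanic.
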(event `/Game/Blueprints/Interaction_Interface.Interact`
  (params (HitVector :type "Vector Structure") (HitActor :type "ActorComponent Object Reference"))
  (bind _returnvalue_location (`KismetMathLibrary.BreakTransform` (`self.GetTransform` self)))
  (`KismetSystemLibrary.PrintString` (`KismetStringLibrary.Conv_IntToString` (`self.GambleNumber`)))
  (bind _asfpschar_v_0_3 (cast `/Game/Blueprints/FPSChar_V_0_3` (`GameplayStatics.GetPlayerPawn` 0)))
  (if (and (>= (`/Game/Blueprints/FPSChar_V_0_3.Currency` _asfpschar_v_0_3) (`self.Price`)) (< (`self.GambleNumber`) (`self.MaxGamble`)))
    (set `self.GambleNumber` (+ (`self.GambleNumber`) 1))
    (set `/Game/Blueprints/FPSChar_V_0_3.Currency` (- (`/Game/Blueprints/FPSChar_V_0_3.Currency` _asfpschar_v_0_3) (`self.Price`)) _asfpschar_v_0_3)
    (set `self.Price` (* (`self.Price`) (`self.PriceMultiply`)))
    (if (<= (`KismetMathLibrary.RandomFloatInRange` 0.0 1.0) (`KismetMathLibrary.FClamp` (+ (`self.ItemChance`) 0.0)))
      (`|SpawnActorFromClass` "/Game/Blueprints/WeightedPicker/ItemSpawn.ItemSpawn_C" (`KismetMathLibrary.MakeTransform` (+ _returnvalue_location (* (`self.GetActorForwardVector` self) 150.0))) "Undefined" "OverrideRootScale" null null)
      (set `self.ItemChance` (`self.StandardItemChance`))
      (else
        (set `self.ItemChance` (+ (`self.ItemChance`) (`self.ChanceIncrease`)))))))

(event `self.ReceiveBeginPlay`
  (`parent.ReceiveBeginPlay`)
  (set `self.ItemChance` (`self.StandardItemChance`)))

(fn `UserConstructionScript`
  (`parent.UserConstructionScript`))