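; Shop automat actor that displays three random items of its Rarity tier and dispenses the one chosen through interaction.
; On BeginPlay, it picks from that tier's item list, spawns the displays at three shop points and sets their Overlap collision to block.
; Interact maps the hit object's name to a slot, spawns a fresh copy at ItemSpawn and destroys all three displays, with no cost check in this graph.
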(event `self.ReceiveBeginPlay`
  (bind _rareitems (`self.RareItems`))
  (bind _epicitems (`self.EpicItems`))
  (bind _legendaryitems (`self.LegendaryItems`))
  (bind _commonitems (`self.CommonItems`))
  (bind _uncommonitems (`self.UncommonItems`))
  (`parent.ReceiveBeginPlay`)
  (switch `/Game/ItemSystem/Enums/ERarity` (`self.Rarity`)
    (:`NewEnumerator0`
      (`self.SpawnShopItems` (`KismetArrayLibrary.Array_Random` _commonitems) (`KismetArrayLibrary.Array_Random` _commonitems) (`KismetArrayLibrary.Array_Random` _commonitems)))
    (:`NewEnumerator1`
      (`self.SpawnShopItems` (`KismetArrayLibrary.Array_Random` _uncommonitems) (`KismetArrayLibrary.Array_Random` _uncommonitems) (`KismetArrayLibrary.Array_Random` _uncommonitems)))
    (:`NewEnumerator2`
      (`self.SpawnShopItems` (`KismetArrayLibrary.Array_Random` _rareitems) (`KismetArrayLibrary.Array_Random` _rareitems) (`KismetArrayLibrary.Array_Random` _rareitems)))
    (:`NewEnumerator3`
      (`self.SpawnShopItems` (`KismetArrayLibrary.Array_Random` _epicitems) (`KismetArrayLibrary.Array_Random` _epicitems) (`KismetArrayLibrary.Array_Random` _epicitems)))
    (:`NewEnumerator4`
      (`self.SpawnShopItems` (`KismetArrayLibrary.Array_Random` _legendaryitems) (`KismetArrayLibrary.Array_Random` _legendaryitems) (`KismetArrayLibrary.Array_Random` _legendaryitems)))))

(event `/Game/Blueprints/Interaction_Interface.Interact`
  (params (HitActor :type "ActorComponent Object Reference"))
  (bind _returnvalue (`SceneComponent.K2_GetComponentLocation` (`self.Item Spawn`)))
  (switch `name` (`KismetStringLibrary.Conv_StringToName` (`KismetSystemLibrary.GetObjectName` HitActor))
    (:`Box`
      (`|SpawnActorFromClass` (`GameplayStatics.GetObjectClass` (`self.Item1`)) (`KismetMathLibrary.MakeTransform` _returnvalue) "Undefined" "OverrideRootScale" null null))
    (:`Box1`
      (`|SpawnActorFromClass` (`GameplayStatics.GetObjectClass` (`self.Item2`)) (`KismetMathLibrary.MakeTransform` _returnvalue) "Undefined" "OverrideRootScale" null null))
    (:`Box2`
      (`|SpawnActorFromClass` (`GameplayStatics.GetObjectClass` (`self.Item3`)) (`KismetMathLibrary.MakeTransform` _returnvalue) "Undefined" "OverrideRootScale" null null)))
  (`self.K2_DestroyActor` (`self.Item1`))
  (`self.K2_DestroyActor` (`self.Item2`))
  (`self.K2_DestroyActor` (`self.Item3`)))

(fn `ChangeCollision`
  (params (Item :type "/Game/Blueprints/WeightedPicker/WeightedItem Object Reference"))
  (bind _overlap (`/Game/Blueprints/WeightedPicker/WeightedItem.Overlap` Item))
  (`PrimitiveComponent.SetCollisionResponseToChannel` _overlap "ECC_WorldStatic" "ECR_Block")
  (`PrimitiveComponent.SetCollisionResponseToChannel` _overlap "ECC_WorldDynamic" "ECR_Block")
  (`PrimitiveComponent.SetCollisionResponseToChannel` _overlap "ECC_Pawn" "ECR_Block")
  (`PrimitiveComponent.SetCollisionResponseToChannel` _overlap "ECC_PhysicsBody" "ECR_Block")
  (`PrimitiveComponent.SetCollisionResponseToChannel` _overlap "ECC_Vehicle" "ECR_Block")
  (`PrimitiveComponent.SetCollisionResponseToChannel` _overlap "ECC_Destructible" "ECR_Block"))

(fn `SpawnShopItems`
  (params (Item1 :type "/Game/Blueprints/WeightedPicker/WeightedItem Class Reference") (Item2 :type "/Game/Blueprints/WeightedPicker/WeightedItem Class Reference") (Item3 :type "/Game/Blueprints/WeightedPicker/WeightedItem Class Reference"))
  (bind _returnvalue (`|SpawnActorFromClass` Item1 (`KismetMathLibrary.MakeTransform` (`SceneComponent.K2_GetComponentLocation` (`self.ShopSpawn1`))) "Undefined" "OverrideRootScale" self null))
  (bind _output_get (set `self.Item1` _returnvalue))
  (`self.ChangeCollision` _output_get)
  (bind _returnvalue_2 (`|SpawnActorFromClass` Item2 (`KismetMathLibrary.MakeTransform` (`SceneComponent.K2_GetComponentLocation` (`self.ShopSpawn2`))) "Undefined" "OverrideRootScale" self null))
  (bind _output_get_2 (set `self.Item2` _returnvalue_2))
  (`self.ChangeCollision` _output_get_2)
  (bind _returnvalue_3 (`|SpawnActorFromClass` Item3 (`KismetMathLibrary.MakeTransform` (`SceneComponent.K2_GetComponentLocation` (`self.ShopSpawn3`))) "Undefined" "OverrideRootScale" self null))
  (bind _output_get_3 (set `self.Item3` _returnvalue_3))
  (`self.ChangeCollision` _output_get_3))

(fn `UserConstructionScript`
  (`parent.UserConstructionScript`))