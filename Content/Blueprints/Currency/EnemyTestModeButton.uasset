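; EnemyTestModeButton is an interactable button that switches a set of enemies to a test mode.
; On Interact, it loops through EnemyList and sets each enemy's TestMode to one fixed enum value, with no toggle back.
; BeginPlay, overlap and Tick are disabled stubs, and the construction script only calls its parent.
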(event `self.Interact`
  (params (HitActor :type "ActorComponent Object Reference"))
  (for _array_element (`self.EnemyList`)
    (set `/Game/Blueprints/Enemy/BP_Enemy.TestMode` "NewEnumerator0" _array_element)))

(fn `UserConstructionScript`
  (`parent.UserConstructionScript`))