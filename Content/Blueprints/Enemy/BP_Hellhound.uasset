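; BP_Hellhound is a hellhound enemy Blueprint that adds dismemberment and attack animation hooks to its parent class.
; Dismember clears the master pose on the front and back skeletal mesh pieces, then turns them into physics-only ragdolls, provided the mesh runs ABP_HellHound.
; AttackAnimation calls the parent version, then sets the Attacking flag on ABP_HellHound to drive the animation.
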(event `self.ReceiveBeginPlay`
  (`parent.ReceiveBeginPlay`))

(event `self.Dismember`
  (bind _sk_hellhoundback (`self.SK_HellhoundBack`))
  (cast `/Game/Geometry/Hellhound_v2/ABP_HellHound` (`SkeletalMeshComponent.GetAnimInstance` (`self.Mesh`)))
  (`SkinnedMeshComponent.SetLeaderPoseComponent` _sk_hellhoundback null false)
  (`SkinnedMeshComponent.SetLeaderPoseComponent` (`self.SK_HellhoundFront`) null false)
  (`PrimitiveComponent.SetSimulatePhysics` _sk_hellhoundback true)
  (`PrimitiveComponent.SetSimulatePhysics` (`self.SK_HellhoundFront`) true)
  (`PrimitiveComponent.SetCollisionEnabled` (`self.SK_HellhoundFront`) "PhysicsOnly")
  (`PrimitiveComponent.SetCollisionEnabled` _sk_hellhoundback "PhysicsOnly"))

(event `self.Attack animation`
  (`parent.Attack animation`)
  (bind _asabp_hell_hound (cast `/Game/Geometry/Hellhound_v2/ABP_HellHound` (`SkeletalMeshComponent.GetAnimInstance` (`self.Mesh`))))
  (set `/Game/Geometry/Hellhound_v2/ABP_HellHound.Attacking` true _asabp_hell_hound))

(fn `UserConstructionScript`
  (`parent.UserConstructionScript`))