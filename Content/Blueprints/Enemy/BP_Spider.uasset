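; Spider enemy Blueprint with a body built from separate skeletal meshes for the torso and legs, extending a parent class.
; On BeginPlay the parts follow the body mesh through master pose.
; The attack event runs the parent logic, then sets the Attacking flag on the ABP_SpiderV2 anim instance.
; Dismember clears the master pose and switches every part to simulated physics with physics-only collision, so they move as independent bodies.
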(event `self.ReceiveBeginPlay`
  (`parent.ReceiveBeginPlay`)
  (`SkinnedMeshComponent.SetLeaderPoseComponent` (`self.SM_Spider_BackL2`) (`self.SM_Spider_Body`) false)
  (`SkinnedMeshComponent.SetLeaderPoseComponent` (`self.SM_Spider_BackR`) (`self.SM_Spider_Body`) false)
  (`SkinnedMeshComponent.SetLeaderPoseComponent` (`self.SM_Spider_BackR2`) (`self.SM_Spider_Body`) false)
  (`SkinnedMeshComponent.SetLeaderPoseComponent` (`self.SM_Spider_BackL`) (`self.SM_Spider_Body`) false)
  (`SkinnedMeshComponent.SetLeaderPoseComponent` (`self.SM_Spider_FrontL`) (`self.SM_Spider_Body`) false)
  (`SkinnedMeshComponent.SetLeaderPoseComponent` (`self.SM_Spider_FrontL2`) (`self.SM_Spider_Body`) false)
  (`SkinnedMeshComponent.SetLeaderPoseComponent` (`self.SM_Spider_FrontR`) (`self.SM_Spider_Body`) false)
  (`SkinnedMeshComponent.SetLeaderPoseComponent` (`self.SM_Spider_Body`) (`self.SM_Spider_Body`) false)
  (`SkinnedMeshComponent.SetLeaderPoseComponent` (`self.SM_Spider_FrontR2`) (`self.SM_Spider_Body`) false))

(event `self.Attack animation`
  (`parent.Attack animation`)
  (bind _asabp_spider_v2 (cast `/Game/Animation/SpiderV2/ABP_SpiderV2` (`SkeletalMeshComponent.GetAnimInstance` (`self.Mesh`))))
  (set `/Game/Animation/SpiderV2/ABP_SpiderV2.Attacking` true _asabp_spider_v2))

(event `self.Dismember`
  (`SkinnedMeshComponent.SetLeaderPoseComponent` (`self.SM_Spider_BackL2`) null false)
  (`SkinnedMeshComponent.SetLeaderPoseComponent` (`self.SM_Spider_BackR`) null false)
  (`SkinnedMeshComponent.SetLeaderPoseComponent` (`self.SM_Spider_BackR2`) null false)
  (`SkinnedMeshComponent.SetLeaderPoseComponent` (`self.SM_Spider_BackL`) null false)
  (`SkinnedMeshComponent.SetLeaderPoseComponent` (`self.SM_Spider_FrontL`) null false)
  (`SkinnedMeshComponent.SetLeaderPoseComponent` (`self.SM_Spider_FrontL2`) null false)
  (`SkinnedMeshComponent.SetLeaderPoseComponent` (`self.SM_Spider_FrontR`) null false)
  (`SkinnedMeshComponent.SetLeaderPoseComponent` (`self.SM_Spider_Body`) null false)
  (`SkinnedMeshComponent.SetLeaderPoseComponent` (`self.SM_Spider_FrontR2`) null false)
  (`PrimitiveComponent.SetSimulatePhysics` (`self.SM_Spider_BackL2`) true)
  (`PrimitiveComponent.SetSimulatePhysics` (`self.SM_Spider_BackR`) true)
  (`PrimitiveComponent.SetSimulatePhysics` (`self.SM_Spider_BackR2`) true)
  (`PrimitiveComponent.SetSimulatePhysics` (`self.SM_Spider_BackL`) true)
  (`PrimitiveComponent.SetSimulatePhysics` (`self.SM_Spider_FrontL`) true)
  (`PrimitiveComponent.SetSimulatePhysics` (`self.SM_Spider_FrontL2`) true)
  (`PrimitiveComponent.SetSimulatePhysics` (`self.SM_Spider_FrontR`) true)
  (`PrimitiveComponent.SetSimulatePhysics` (`self.SM_Spider_Body`) true)
  (`PrimitiveComponent.SetSimulatePhysics` (`self.SM_Spider_FrontR2`) true)
  (`PrimitiveComponent.SetCollisionEnabled` (`self.SM_Spider_BackL2`) "PhysicsOnly")
  (`PrimitiveComponent.SetCollisionEnabled` (`self.SM_Spider_BackR`) "PhysicsOnly")
  (`PrimitiveComponent.SetCollisionEnabled` (`self.SM_Spider_BackR2`) "PhysicsOnly")
  (`PrimitiveComponent.SetCollisionEnabled` (`self.SM_Spider_BackL`) "PhysicsOnly")
  (`PrimitiveComponent.SetCollisionEnabled` (`self.SM_Spider_FrontL`) "PhysicsOnly")
  (`PrimitiveComponent.SetCollisionEnabled` (`self.SM_Spider_FrontL2`) "PhysicsOnly")
  (`PrimitiveComponent.SetCollisionEnabled` (`self.SM_Spider_FrontR`) "PhysicsOnly")
  (`PrimitiveComponent.SetCollisionEnabled` (`self.SM_Spider_Body`) "PhysicsOnly")
  (`PrimitiveComponent.SetCollisionEnabled` (`self.SM_Spider_FrontR2`) "PhysicsOnly"))

(fn `UserConstructionScript`
  (`parent.UserConstructionScript`))