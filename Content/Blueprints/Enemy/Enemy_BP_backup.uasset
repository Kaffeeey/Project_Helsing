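; Enemy character Blueprint with HP, AI perception and projectile shooting; death destroys it and refills the player's potion.
; Tick counts a cooldown up to FireRate, gating FireBullet, which spawns Wurm_Projectile_BP at BulletPoint.
; StartShooting calls an empty Attack, likely an override hook, so nothing here calls FireBullet.
; Perception updates write CanSeePlayer to the Blackboard, but only when the sensed actor casts to Enemy_BP.
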(event `self.ReceiveBeginPlay`
  (set `self.MomFireRate` (`self.FireRate`))
  (set `self.CanFire` true))

(event `StartShooting`
  (`self.Attack`))

(event `StopShooting`)

(event `self.ReceiveTick`
  (params (DeltaSeconds :type "Float (single-precision)"))
  (if (< (`self.MomFireRate`) (`self.FireRate`))
    (set `self.MomFireRate` (+ (`self.MomFireRate`) (`GameplayStatics.GetWorldDeltaSeconds`)))
    (if (>= (`self.MomFireRate`) (`self.FireRate`))
      (set `self.MomFireRate` (`self.FireRate`))
      (set `self.CanFire` true))))

(event `self.AIPerception.OnTargetPerceptionUpdated`
  (params (Actor :type "Actor Object Reference") (Stimulus :type "AIStimulus Structure"))
  (cast `/Game/Blueprints/Enemy/Enemy_BP` Actor)
  (`BlackboardComponent.SetValueAsBool` (`AIBlueprintHelperLibrary.GetBlackboard` null) "CanSeePlayer" Stimulus_bSuccessfullySensed))

(fn `Attack`)

(fn `FireBullet`
  (if (`self.CanFire`)
    (`|SpawnActorFromClass` "/Game/Blueprints/Wurm_Projectile_BP.Wurm_Projectile_BP_C" (`KismetMathLibrary.MakeTransform` (`SceneComponent.K2_GetComponentLocation` (`self.BulletPoint`)) (`SceneComponent.GetSocketRotation` (`self.CapsuleComponent`) "None")) "Undefined" "OverrideRootScale" null null)
    (set `self.CanFire` false)
    (set `self.MomFireRate` 0.0)))

(fn `GetDamage`
  (params (Damage :type "Float (double-precision)") (HitPosition :type "Vector Structure") (HitActor :type "Actor Object Reference"))
  (set `self.HP` (- (`self.HP`) Damage))
  (if (<= (`self.HP`) 0.0)
    (`self.K2_DestroyActor`)
    (bind _asfpschar_v_0_3 (cast `/Game/Blueprints/FPSChar_V_0_3` (`GameplayStatics.GetPlayerCharacter` 0))
      (:`then`
        (`/Game/Blueprints/FPSChar_V_0_3.FillPotion` _asfpschar_v_0_3))
      (:`CastFailed`
        (`self.K2_DestroyActor`)))))

(fn `UserConstructionScript`)