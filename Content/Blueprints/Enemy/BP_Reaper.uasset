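; Reaper enemy Blueprint with five montage attacks, built on a parent class.
; Each attack event fires once MomFireRate reaches FireRate, then sets the next cooldown to montage length plus AttackTime and resets the timer.
; Tick counts down the montage time to clear IsAttacking.
; PathJumpCheck sphere-scans AI path points for NavLinkProxy actors but takes no action on finding one.
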(event `self.ReceiveTick`
  (params (DeltaSeconds :type "Float (single-precision)"))
  (`parent.ReceiveTick` DeltaSeconds)
  (if (> (`self.AnimTime`) 0.0)
    (set `self.AnimTime` (- (`self.AnimTime`) (`GameplayStatics.GetWorldDeltaSeconds`)))
    (else
      (set `self.IsAttacking` false))))

(event `Attack1`
  (if (>= (`self.MomFireRate`) (`self.FireRate`))
    (`self.PlayAnimMontage` (`self.AttackAnim1`))
    (bind _returnvalue (`AnimSequenceBase.GetPlayLength` (`self.AttackAnim1`)))
    (bind _output_get (set `self.AnimTime` _returnvalue))
    (set `self.FireRate` (+ _output_get (`self.AttackTime`)))
    (set `self.MomFireRate` 0.0)
    (set `self.IsAttacking` true)))

(event `Attack2`
  (if (>= (`self.MomFireRate`) (`self.FireRate`))
    (`self.PlayAnimMontage` (`self.AttackAnim2`))
    (bind _returnvalue (`AnimSequenceBase.GetPlayLength` (`self.AttackAnim2`)))
    (bind _output_get (set `self.AnimTime` _returnvalue))
    (set `self.FireRate` (+ _output_get (`self.AttackTime`)))
    (set `self.MomFireRate` 0.0)
    (set `self.IsAttacking` true)))

(event `Attack3`
  (if (>= (`self.MomFireRate`) (`self.FireRate`))
    (`self.PlayAnimMontage` (`self.AttackAnim3`))
    (bind _returnvalue (`AnimSequenceBase.GetPlayLength` (`self.AttackAnim3`)))
    (bind _output_get (set `self.AnimTime` _returnvalue))
    (set `self.FireRate` (+ _output_get (`self.AttackTime`)))
    (set `self.MomFireRate` 0.0)
    (set `self.IsAttacking` true)))

(event `Attack4`
  (if (>= (`self.MomFireRate`) (`self.FireRate`))
    (`self.PlayAnimMontage` (`self.AttackAnim4`))
    (bind _returnvalue (`AnimSequenceBase.GetPlayLength` (`self.AttackAnim4`)))
    (bind _output_get (set `self.AnimTime` _returnvalue))
    (set `self.FireRate` (+ _output_get (`self.AttackTime`)))
    (set `self.MomFireRate` 0.0)
    (set `self.IsAttacking` true)))

(event `Attack5`
  (if (>= (`self.MomFireRate`) (`self.FireRate`))
    (`self.PlayAnimMontage` (`self.AttackAnim5`))
    (bind _returnvalue (`AnimSequenceBase.GetPlayLength` (`self.AttackAnim5`)))
    (bind _output_get (set `self.AnimTime` _returnvalue))
    (set `self.FireRate` (+ _output_get (`self.AttackTime`)))
    (set `self.MomFireRate` 0.0)
    (set `self.IsAttacking` true)))

(event `PathJumpCheck`
  (for _array_element (`AIBlueprintHelperLibrary.GetCurrentPathPoints` (`AIBlueprintHelperLibrary.GetAIController` null)) :!label _label
    (bind _outactors (`KismetSystemLibrary.SphereOverlapActors` _array_element 50.0 (`self.Object Types`)))
    (for _array_element_2 _outactors
      (cast `NavLinkProxy` _array_element_2)
      (goto _label :!via `Break`))))

(fn `UserConstructionScript`
  (`parent.UserConstructionScript`))