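; FlyEnemyTest is a test flying enemy that senses whether the player is within fighting range or personal space for its AI.
; Every eighth tick it fires a FixedUpdate event that runs DistanceCheck for both radii.
; DistanceCheck uses a sphere overlap filtered to the FPS player character.
; The results are stored and written as bools to the AI controller's Blackboard, presumably for behavior tree decisions.
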(event `self.ReceiveTick`
  (params (DeltaSeconds :type "Float (single-precision)"))
  (`parent.ReceiveTick` DeltaSeconds)
  (set `self.FixedUpdateCount` (+ (`self.FixedUpdateCount`) 1))
  (if (>= (`self.FixedUpdateCount`) 8)
    (`self.FixedUpdate`)
    (set `self.FixedUpdateCount` 0)))

(event `FixedUpdate`
  (bind _returnvalue (`AIBlueprintHelperLibrary.GetBlackboard` (`AIBlueprintHelperLibrary.GetAIController` self)))
  (bind _playercheck (`self.DistanceCheck` (`self.FightingRange`)))
  (set `self.PlayerInRange` _playercheck)
  (bind _playercheck_2 (`self.DistanceCheck` (`self.PersonalSpace`)))
  (set `self.PlayerInPersonalSpace` _playercheck_2)
  (`BlackboardComponent.SetValueAsBool` _returnvalue "PlayerInRange" (`self.PlayerInRange`))
  (`BlackboardComponent.SetValueAsBool` _returnvalue "PlayerInPersonalSpace" (`self.PlayerInPersonalSpace`)))

(fn `DistanceCheck`
  (params (Distance :type "Float (double-precision)"))
  (returns (PlayerCheck :type Boolean))
  (bind _outactors (`KismetSystemLibrary.SphereOverlapActors` (`self.K2_GetActorLocation` self) Distance (`self.Object Types`) "/Game/Blueprints/FPSChar_V_0_3.FPSChar_V_0_3_C"))
  (for _array_element _outactors
    (cast `/Game/Blueprints/FPSChar_V_0_3` _array_element)
    (return true))
  (return false))

(fn `UserConstructionScript`
  (`parent.UserConstructionScript`))