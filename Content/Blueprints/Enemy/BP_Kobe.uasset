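; BP_Kobe is a flying gargoyle enemy built on BP_Enemy.
; On BeginPlay it sets its max fly speed from the class-default Speed, and AttackAnimation raises the Attack flag on ABP_Gargoyle.
; Dismember fakes a breakup by hiding the main mesh and revealing separate body-part components with physics simulation and physics-only collision.
; A master-pose hookup for those parts is left unconnected and never runs.
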(event `self.ReceiveBeginPlay`
  (`parent.ReceiveBeginPlay`)
  (bind _asbp_enemy (cast `/Game/Blueprints/Enemy/BP_Enemy` self))
  (set `CharacterMovementComponent.MaxFlySpeed` (`.Speed` (defaults `Object` (`GameplayStatics.GetObjectClass` _asbp_enemy))) (`self.CharacterMovement`)))

(event `/Game/Blueprints/Enemy/BP_Enemy.Attack animation`
  (bind _asabp_gargoyle (cast `/Game/Geometry/Gargoyle/ABP_Gargoyle` (`SkeletalMeshComponent.GetAnimInstance` (`self.Mesh`))))
  (set `/Game/Geometry/Gargoyle/ABP_Gargoyle.Attack` true _asabp_gargoyle))

(event `self.ReceiveTick`
  (params (DeltaSeconds :type "Float (single-precision)"))
  (`parent.ReceiveTick` DeltaSeconds))

(event `/Game/Blueprints/Enemy/BP_Enemy.Dismember`
  (`SceneComponent.SetVisibility` (`self.Mesh`) false false)
  (`SceneComponent.SetVisibility` (`self.RAW_Gargoyle_WingR`) true false)
  (`SceneComponent.SetVisibility` (`self.RAW_Gargoyle_lowerLegR`) true false)
  (`SceneComponent.SetVisibility` (`self.RAW_Gargoyle_head`) true false)
  (`SceneComponent.SetVisibility` (`self.RAW_Gargoyle_hornL`) true false)
  (`SceneComponent.SetVisibility` (`self.RAW_Gargoyle_hornR`) true false)
  (`SceneComponent.SetVisibility` (`self.RAW_Gargoyle_lowerArmL`) true false)
  (`SceneComponent.SetVisibility` (`self.RAW_Gargoyle_lowerArmR`) true false)
  (`SceneComponent.SetVisibility` (`self.RAW_Gargoyle_lowerLegL`) true false)
  (`SceneComponent.SetVisibility` (`self.RAW_Gargoyle_body`) true false)
  (`SceneComponent.SetVisibility` (`self.RAW_Gargoyle_Tail`) true false)
  (`SceneComponent.SetVisibility` (`self.RAW_Gargoyle_UpperArmL`) true false)
  (`SceneComponent.SetVisibility` (`self.RAW_Gargoyle_UpperArmR`) true false)
  (`SceneComponent.SetVisibility` (`self.RAW_Gargoyle_UpperLegL`) true false)
  (`SceneComponent.SetVisibility` (`self.RAW_Gargoyle_UpperLegR`) true false)
  (`SceneComponent.SetVisibility` (`self.RAW_Gargoyle_WingL`) true false)
  (`PrimitiveComponent.SetSimulatePhysics` (`self.RAW_Gargoyle_lowerLegR`) true)
  (`PrimitiveComponent.SetSimulatePhysics` (`self.RAW_Gargoyle_head`) true)
  (`PrimitiveComponent.SetSimulatePhysics` (`self.RAW_Gargoyle_hornL`) true)
  (`PrimitiveComponent.SetSimulatePhysics` (`self.RAW_Gargoyle_hornR`) true)
  (`PrimitiveComponent.SetSimulatePhysics` (`self.RAW_Gargoyle_lowerArmL`) true)
  (`PrimitiveComponent.SetSimulatePhysics` (`self.RAW_Gargoyle_lowerArmR`) true)
  (`PrimitiveComponent.SetSimulatePhysics` (`self.RAW_Gargoyle_lowerLegL`) true)
  (`PrimitiveComponent.SetSimulatePhysics` (`self.RAW_Gargoyle_body`) true)
  (`PrimitiveComponent.SetSimulatePhysics` (`self.RAW_Gargoyle_Tail`) true)
  (`PrimitiveComponent.SetSimulatePhysics` (`self.RAW_Gargoyle_UpperArmL`) true)
  (`PrimitiveComponent.SetSimulatePhysics` (`self.RAW_Gargoyle_UpperArmR`) true)
  (`PrimitiveComponent.SetSimulatePhysics` (`self.RAW_Gargoyle_UpperLegL`) true)
  (`PrimitiveComponent.SetSimulatePhysics` (`self.RAW_Gargoyle_UpperLegR`) true)
  (`PrimitiveComponent.SetSimulatePhysics` (`self.RAW_Gargoyle_WingL`) true)
  (`PrimitiveComponent.SetSimulatePhysics` (`self.RAW_Gargoyle_WingR`) true)
  (`PrimitiveComponent.SetCollisionEnabled` (`self.RAW_Gargoyle_lowerLegR`) "PhysicsOnly")
  (`PrimitiveComponent.SetCollisionEnabled` (`self.RAW_Gargoyle_head`) "PhysicsOnly")
  (`PrimitiveComponent.SetCollisionEnabled` (`self.RAW_Gargoyle_hornL`) "PhysicsOnly")
  (`PrimitiveComponent.SetCollisionEnabled` (`self.RAW_Gargoyle_hornR`) "PhysicsOnly")
  (`PrimitiveComponent.SetCollisionEnabled` (`self.RAW_Gargoyle_lowerArmL`) "PhysicsOnly")
  (`PrimitiveComponent.SetCollisionEnabled` (`self.RAW_Gargoyle_lowerArmR`) "PhysicsOnly")
  (`PrimitiveComponent.SetCollisionEnabled` (`self.RAW_Gargoyle_lowerLegL`) "PhysicsOnly")
  (`PrimitiveComponent.SetCollisionEnabled` (`self.RAW_Gargoyle_body`) "PhysicsOnly")
  (`PrimitiveComponent.SetCollisionEnabled` (`self.RAW_Gargoyle_Tail`) "PhysicsOnly")
  (`PrimitiveComponent.SetCollisionEnabled` (`self.RAW_Gargoyle_UpperArmL`) "PhysicsOnly")
  (`PrimitiveComponent.SetCollisionEnabled` (`self.RAW_Gargoyle_UpperArmR`) "PhysicsOnly")
  (`PrimitiveComponent.SetCollisionEnabled` (`self.RAW_Gargoyle_UpperLegL`) "PhysicsOnly")
  (`PrimitiveComponent.SetCollisionEnabled` (`self.RAW_Gargoyle_UpperLegR`) "PhysicsOnly")
  (`PrimitiveComponent.SetCollisionEnabled` (`self.RAW_Gargoyle_WingL`) "PhysicsOnly")
  (`PrimitiveComponent.SetCollisionEnabled` (`self.RAW_Gargoyle_WingR`) "PhysicsOnly"))

(fn `UserConstructionScript`
  (`parent.UserConstructionScript`))