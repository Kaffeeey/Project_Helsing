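; BP_Harald is an enemy Blueprint that adds Harald-specific attack animation and dismemberment to its parent class.
; Attacks run the parent logic, then set the Attacking flag on the ABP_Haraldv2 anim instance.
; Dismember hides the main mesh and reveals ten separate body-part components, switching them to physics simulation with physics-only collision so the body breaks apart.
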(event `self.ReceiveBeginPlay`
  (`parent.ReceiveBeginPlay`))

(event `self.Attack animation`
  (`parent.Attack animation`)
  (bind _asabp_haraldv_2 (cast `/Game/Animation/Harald/v2/ABP_Haraldv2` (`SkeletalMeshComponent.GetAnimInstance` (`self.Mesh`))))
  (set `/Game/Animation/Harald/v2/ABP_Haraldv2.Attacking` true _asabp_haraldv_2))

(event `self.Dismember`
  (`PrimitiveComponent.SetSimulatePhysics` (`self.RAW_Harald_clawL`) true)
  (`PrimitiveComponent.SetSimulatePhysics` (`self.RAW_Harald_clawR`) true)
  (`PrimitiveComponent.SetSimulatePhysics` (`self.RAW_Harald_lowerLegL`) true)
  (`PrimitiveComponent.SetSimulatePhysics` (`self.RAW_Harald_lowerLegR`) true)
  (`PrimitiveComponent.SetSimulatePhysics` (`self.RAW_Harald_upperArmL`) true)
  (`PrimitiveComponent.SetSimulatePhysics` (`self.RAW_Harald_upperArmR`) true)
  (`PrimitiveComponent.SetSimulatePhysics` (`self.RAW_Harald_upperLegR`) true)
  (`PrimitiveComponent.SetSimulatePhysics` (`self.RAW_Harald_upperLegL`) true)
  (`PrimitiveComponent.SetSimulatePhysics` (`self.RAW_Harald_body`) true)
  (`PrimitiveComponent.SetSimulatePhysics` (`self.RAW_Harald_head`) true)
  (`PrimitiveComponent.SetCollisionEnabled` (`self.RAW_Harald_clawL`) "PhysicsOnly")
  (`PrimitiveComponent.SetCollisionEnabled` (`self.RAW_Harald_clawR`) "PhysicsOnly")
  (`PrimitiveComponent.SetCollisionEnabled` (`self.RAW_Harald_lowerLegL`) "PhysicsOnly")
  (`PrimitiveComponent.SetCollisionEnabled` (`self.RAW_Harald_lowerLegR`) "PhysicsOnly")
  (`PrimitiveComponent.SetCollisionEnabled` (`self.RAW_Harald_upperArmL`) "PhysicsOnly")
  (`PrimitiveComponent.SetCollisionEnabled` (`self.RAW_Harald_upperArmR`) "PhysicsOnly")
  (`PrimitiveComponent.SetCollisionEnabled` (`self.RAW_Harald_upperLegR`) "PhysicsOnly")
  (`PrimitiveComponent.SetCollisionEnabled` (`self.RAW_Harald_upperLegL`) "PhysicsOnly")
  (`PrimitiveComponent.SetCollisionEnabled` (`self.RAW_Harald_body`) "PhysicsOnly")
  (`PrimitiveComponent.SetCollisionEnabled` (`self.RAW_Harald_head`) "PhysicsOnly")
  (`SceneComponent.SetVisibility` (`self.Mesh`) false false)
  (`SceneComponent.SetVisibility` (`self.RAW_Harald_clawL`) true false)
  (`SceneComponent.SetVisibility` (`self.RAW_Harald_clawR`) true false)
  (`SceneComponent.SetVisibility` (`self.RAW_Harald_lowerLegL`) true false)
  (`SceneComponent.SetVisibility` (`self.RAW_Harald_lowerLegR`) true false)
  (`SceneComponent.SetVisibility` (`self.RAW_Harald_upperArmL`) true false)
  (`SceneComponent.SetVisibility` (`self.RAW_Harald_upperArmR`) true false)
  (`SceneComponent.SetVisibility` (`self.RAW_Harald_upperLegR`) true false)
  (`SceneComponent.SetVisibility` (`self.RAW_Harald_upperLegL`) true false)
  (`SceneComponent.SetVisibility` (`self.RAW_Harald_body`) true false)
  (`SceneComponent.SetVisibility` (`self.RAW_Harald_head`) true false))

(fn `UserConstructionScript`
  (`parent.UserConstructionScript`))