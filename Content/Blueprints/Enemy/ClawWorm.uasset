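; ClawWorm is an enemy child Blueprint that supplies its own body-region bone sets to logic inherited from its parent.
; On BeginPlay it runs the parent's logic, then copies its child head, torso and limb bone variables into the HeeadBones, TorsoBones and LimbBones variables.
; The construction script only calls the parent, and the overlap and Tick events are disabled.
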(event `self.ReceiveBeginPlay`
  (`parent.ReceiveBeginPlay`)
  (set `self.HeeadBones` (`self.HeadBonesChild`))
  (set `self.TorsoBones` (`self.TortsoBonesChild`))
  (set `self.LimbBones` (`self.LimbBonesChild`)))

(fn `UserConstructionScript`
  (`parent.UserConstructionScript`))