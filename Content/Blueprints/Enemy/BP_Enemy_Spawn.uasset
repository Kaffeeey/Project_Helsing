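; Enemy spawner that creates range or close-combat AI from a class-to-count list, each with its matching behavior tree.
; After an initial batch, every eighth tick prunes invalid enemies and runs timed random bursts or respawns cleared waves.
; Placement uses level-matched, unused spawnpoints with random fallback, or random offsets retried on overlap.
; With a spawn limit, it deactivates once the limit is reached and enemies are gone, starting the linked spawners.
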(event `GetSpawnpoints`
  (bind _outactors (`GameplayStatics.GetAllActorsOfClass` "/Game/Blueprints/Enemy/BP_SpawnpointChild.BP_SpawnpointChild_C"))
  (set `self.SpawnpointList` _outactors))

(event `Start`
  (`self.SetActorTickEnabled` (`self.Active`))
  (bind _keys (`BlueprintMapLibrary.Map_Keys` (`self.EnemyList`)))
  (for _array_element _keys
    (if (not (`KismetSystemLibrary.IsValidClass` _array_element))
      (goto _label :!via `Close`)))
  (`/Engine/EditorBlueprintResources/StandardMacros.Gate` false :!label _label
    (:`Exit`
      (`self.SpawnEnemy`)
      (set `self.tempTime` (`self.SpawnTime`))
      (set `self.tempTimeSpawnNumber` (`self.TimeSpawnNumber`)))))

(event `self.ReceiveBeginPlay`
  (bind _active (`self.Active`))
  (if _active
    (`self.Start`)
    (else
      (`self.SetActorTickEnabled` _active))))

(event `self.ReceiveTick`
  (params (DeltaSeconds :type "Float (single-precision)"))
  (set `self.FixedUpdateCount` (+ (`self.FixedUpdateCount`) 1))
  (if (>= (`self.FixedUpdateCount`) 8)
    (`self.FixedUpdate`)
    (set `self.FixedUpdateCount` 0)))

(event `FixedUpdate`
  (bind _tempspawnpoint (`self.tempSpawnPoint`))
  (bind _tempspawnedenemylist (`self.TempSpawnedEnemyList`))
  (for _array_element _tempspawnedenemylist
    (`/Engine/EditorBlueprintResources/StandardMacros.IsValid` _array_element
      (:`Is Not Valid`
        (`KismetArrayLibrary.Array_RemoveItem` _tempspawnedenemylist _array_element))))
  (if (`self.SpawnLimit`)
    (if (>= (- (`self.MaxEnemySpawn`) 1) (`self.SpawnedEnemies`))
      (switch `/Game/Blueprints/Enemy/Enum_SpawnType` (`self.SpawnType`) :!label _label_2
        (:`NewEnumerator0`
          (if (and (<= (`self.tempTime`) 0.0) (< (`KismetArrayLibrary.Array_Length` (`self.TempSpawnedEnemyList`)) (`self.MaxTimeSpawn`)))
            (if (> (`self.tempTimeSpawnNumber`) 0) :!label _label_3
              (bind _keys (`BlueprintMapLibrary.Map_Keys` (`self.EnemyList`)))
              (bind _outitem (`KismetArrayLibrary.Array_Random` _keys))
              (set `self.NextEnemyToSpawn` _outitem)
              (`self.SetSpawnpoint`)
              (bind _asbp_enemy (castclass `/Game/Blueprints/Enemy/BP_Enemy` _outitem))
              (switch `/Game/Blueprints/Enemy/Enum_Enemy_Type` (`.EnemyType` (defaults `Object` _asbp_enemy))
                (:`NewEnumerator0`
                  (bind _returnvalue (`AIBlueprintHelperLibrary.SpawnAIFromClass` _outitem "/Game/AI/OldAI/RangeAI/BT_RangeEnemy_AI.BT_RangeEnemy_AI" _tempspawnpoint (struct) false null))
                  (`KismetArrayLibrary.Array_Add` (`self.TempSpawnedEnemyList`) _returnvalue))
                (:`NewEnumerator1`
                  (bind _returnvalue_2 (`AIBlueprintHelperLibrary.SpawnAIFromClass` _outitem "/Game/AI/OldAI/CloseCombatAI/BT_CloseCombatEnemy_AI.BT_CloseCombatEnemy_AI" _tempspawnpoint (struct) false null))
                  (`KismetArrayLibrary.Array_Add` (`self.TempSpawnedEnemyList`) _returnvalue_2)))
              (set `self.SpawnedEnemies` (+ (`self.SpawnedEnemies`) 1))
              (set `self.tempTimeSpawnNumber` (- (`self.tempTimeSpawnNumber`) 1))
              (goto _label_3)
              (else
                (set `self.tempTimeSpawnNumber` (`self.TimeSpawnNumber`))
                (set `self.tempTime` (`self.SpawnTime`))))
            (else
              (set `self.tempTime` (- (`self.tempTime`) (`GameplayStatics.GetWorldDeltaSeconds`))))))
        (:`NewEnumerator1`
          (if (<= (`KismetArrayLibrary.Array_Length` (`self.TempSpawnedEnemyList`)) 0)
            (`self.SpawnEnemy`))))
      (elif (<= (`KismetArrayLibrary.Array_Length` (`self.TempSpawnedEnemyList`)) 0)
        (`self.Deactivate`)))
    (else
      (goto _label_2))))

(event `Deactivate`
  (bind _output_get (set `self.Active` false))
  (`self.SetActorTickEnabled` _output_get)
  (if (>= (`KismetArrayLibrary.Array_Length` (`self.NextSpawnList`)) 0)
    (for _array_element (`self.NextSpawnList`)
      (set `/Game/Blueprints/Enemy/BP_Enemy_Spawn.Active` true _array_element)
      (`self.Start` _array_element))))

(fn `SetSpawnpoint`
  (locals (YouShallNotSpawn :type "Array of EObjectTypeQuery Enum"))
  (bind _tempspawnpointlist (`self.TempSpawnpointList`))
  (bind _outitem (`KismetArrayLibrary.Array_Random` _tempspawnpointlist))
  (bind _keys (`BlueprintMapLibrary.Map_Keys` (`self.EnemyList`)))
  (for _array_element _keys
    (if (not (`KismetSystemLibrary.IsValidClass` _array_element))
      (goto _label :!via `Close`)))
  (`/Engine/EditorBlueprintResources/StandardMacros.Gate` false :!label _label
    (:`Exit`
      (if (`self.UseSpawnpoints`)
        (`KismetArrayLibrary.Array_Clear` (`self.TempSpawnpointList`))
        (for _array_element_2 (`self.SpawnpointList`)
          (for _array_element_3 (`/Game/Blueprints/Enemy/BP_SpawnpointChild.EnemyType` _array_element_2)
            (if (and (`|EnumEquality` _array_element_3 (`.EnemyLevel` (defaults `Object` (`self.NextEnemyToSpawn`)))) (<= (`/Game/Blueprints/Enemy/BP_SpawnpointChild.Used` _array_element_2) 0.0))
              (`KismetArrayLibrary.Array_Add` _tempspawnpointlist _array_element_2)
              (set `self.tempSpawnPoint` (`self.K2_GetActorLocation` _outitem))
              (set `self.TempCanSpawn` true)
              (set `/Game/Blueprints/Enemy/BP_SpawnpointChild.Used` 3.0 _outitem)
              (return)
              (else
                (set `self.TempCanSpawn` false)))))
        (if (not (and (`self.TempCanSpawn`) (< (`self.SpawnTime`) 0.0)))
          (set `self.tempSpawnPoint` (`self.K2_GetActorLocation` (`KismetArrayLibrary.Array_Random` (`self.SpawnpointList`))))
          (return))
        (else
          (bind _output_get (set `self.tempSpawnPoint` (+ (`self.SpawnPoint`) (`KismetMathLibrary.MakeVector` (`KismetMathLibrary.RandomFloatInRange` -250.0 250.0) (`KismetMathLibrary.RandomFloatInRange` -250.0 250.0)))))
          (bind _outactors (`KismetSystemLibrary.SphereOverlapActors` (+ _output_get (0.0 0.0 150.0)) 1.5 (`local.YouShallNotSpawn`)))
          (if (> (`KismetArrayLibrary.Array_Length` _outactors) 0)
            (`self.SetSpawnpoint`)))))))

(fn `SpawnEnemy`
  (bind _tempspawnpoint (`self.tempSpawnPoint`))
  (bind _enemylist (`self.EnemyList`))
  (bind _keys (`BlueprintMapLibrary.Map_Keys` _enemylist))
  (for _array_element _keys
    (set `self.NextEnemyToSpawn` _array_element)
    (bind _output_get (set `self.tempSpawnNumber` (`BlueprintMapLibrary.Map_Find` _enemylist _array_element)))
    (if (> _output_get 0)
      (`self.SetSpawnpoint` :!label _label)
      (bind _asbp_enemy (castclass `/Game/Blueprints/Enemy/BP_Enemy` _array_element))
      (switch `/Game/Blueprints/Enemy/Enum_Enemy_Type` (`.EnemyType` (defaults `Object` _asbp_enemy))
        (:`NewEnumerator0`
          (bind _returnvalue (`AIBlueprintHelperLibrary.SpawnAIFromClass` _array_element "/Game/AI/OldAI/RangeAI/BT_RangeEnemy_AI.BT_RangeEnemy_AI" _tempspawnpoint (struct) false null))
          (`KismetArrayLibrary.Array_Add` (`self.TempSpawnedEnemyList`) _returnvalue))
        (:`NewEnumerator1`
          (bind _returnvalue_2 (`AIBlueprintHelperLibrary.SpawnAIFromClass` _array_element "/Game/AI/OldAI/CloseCombatAI/BT_CloseCombatEnemy_AI.BT_CloseCombatEnemy_AI" _tempspawnpoint (struct) false null))
          (`KismetArrayLibrary.Array_Add` (`self.TempSpawnedEnemyList`) _returnvalue_2)))
      (`KismetSystemLibrary.PrintString` "EnemySpawned")
      (set `self.SpawnedEnemies` (+ (`self.SpawnedEnemies`) 1))
      (if (> (`self.tempSpawnNumber`) 1)
        (set `self.tempSpawnNumber` (- (`self.tempSpawnNumber`) 1))
        (goto _label)))))

(fn `UserConstructionScript`
  (`self.GetSpawnpoints`))