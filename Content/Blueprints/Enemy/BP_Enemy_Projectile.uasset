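; Enemy projectile actor that damages the player character, FPSChar_V_0_3, on contact.
; On Hit, it passes its Damage and a fixed enum value to the character's TakeDamage, and destroys itself whatever it struck.
; Actor overlap with the player applies the same damage but does not destroy the projectile.
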(event `self.ReceiveBeginPlay`)

(event `self.ReceiveTick`
  (params (DeltaSeconds :type "Float (single-precision)")))

(event `self.ReceiveHit`
  (params (MyComp :type "PrimitiveComponent Object Reference") (Other :type "Actor Object Reference") (OtherComp :type "PrimitiveComponent Object Reference") (bSelfMoved :type Boolean) (HitLocation :type "Vector Structure") (HitNormal :type "Vector Structure") (NormalImpulse :type "Vector Structure") (Hit :type "HitResult Structure (by ref)"))
  (bind _asfpschar_v_0_3 (cast `/Game/Blueprints/FPSChar_V_0_3` Other)
    (:`then`
      (`/Game/Blueprints/FPSChar_V_0_3.TakeDamage` _asfpschar_v_0_3 (`self.Damage`) "NewEnumerator0")
      (`self.K2_DestroyActor`))
    (:`CastFailed`
      (`self.K2_DestroyActor`))))

(event `self.ReceiveActorBeginOverlap`
  (params (OtherActor :type "Actor Object Reference"))
  (bind _asfpschar_v_0_3 (cast `/Game/Blueprints/FPSChar_V_0_3` OtherActor))
  (`/Game/Blueprints/FPSChar_V_0_3.TakeDamage` _asfpschar_v_0_3 (`self.Damage`) "NewEnumerator0"))

(fn `UserConstructionScript`
  (`parent.UserConstructionScript`))