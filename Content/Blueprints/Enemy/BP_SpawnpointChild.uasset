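; Enemy spawn point actor that carries a spawn number and a "Used" timer.
; Its construction script, when its number is not yet in its own list, scans all BP_SpawnpointChild actors, merges their number lists and bumps SpawnNumber past existing ones, capped by the actor count.
; Tick counts Used down by delta time while it is above zero, acting as a cooldown set outside this graph.
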(event `self.ReceiveTick`
  (params (DeltaSeconds :type "Float (single-precision)"))
  (if (> (`self.Used`) 0.0)
    (set `self.Used` (- (`self.Used`) DeltaSeconds))))

(fn `UserConstructionScript`
  (bind _spawnnumberlist (`self.SpawnNumberList`))
  (if (not (`KismetArrayLibrary.Array_Contains` (`self.SpawnNumberList`) (`self.SpawnNumber`)))
    (bind _outactors (`GameplayStatics.GetAllActorsOfClass` "BP_SpawnpointChild_C"))
    (for _array_element _outactors
      (for _array_element_2 (`/Game/Blueprints/Enemy/BP_SpawnpointChild.SpawnNumberList` _array_element)
        (if (not (`KismetArrayLibrary.Array_Contains` _spawnnumberlist _array_element_2))
          (`KismetArrayLibrary.Array_Add` _spawnnumberlist _array_element_2)))
      (bind _spawnnumber (`/Game/Blueprints/Enemy/BP_SpawnpointChild.SpawnNumber` _array_element))
      (bind _returnvalue (+ _spawnnumber 1))
      (if (and (<= (`self.SpawnNumber`) _spawnnumber) (< (`self.SpawnNumber`) (`KismetArrayLibrary.Array_Length` _outactors)) (not (`KismetArrayLibrary.Array_Contains` (`self.SpawnNumberList`) _returnvalue)))
        (bind _output_get (set `self.SpawnNumber` _returnvalue))
        (`KismetArrayLibrary.Array_Add` (`self.SpawnNumberList`) _output_get)))))