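; Enemy spawner that populates an area with AI enemies, either on a timer or in waves.
; BeginPlay spawns every EnemyList class in its mapped count at random XY offsets around SpawnPoint.
; Tick prunes invalid enemies, then either spawns timed batches of random classes while below MaxTimeSpawn, or respawns the full list once all are gone.
; Each class default EnemyType selects the ranged or close-combat behavior tree.
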(event `self.ReceiveBeginPlay`
  (`self.SpawnEnemy`)
  (set `self.tempTime` (`self.SpwanTime`))
  (set `self.tempTimeSpawnNumber` (`self.TimeSpawnNumber`)))

(event `self.ReceiveTick`
  (params (DeltaSeconds :type "Float (single-precision)"))
  (bind _tempspawnpoint (`self.tempSpawnPoint`))
  (bind _spawnedenemylist (`self.SpawnedEnemyList`))
  (bind _spawnedenemylist_2 (`self.SpawnedEnemyList`))
  (switch `/Game/Blueprints/Enemy/SpawnType_Enum` (`self.SpawnType`)
    (:`NewEnumerator0`
      (for _array_element _spawnedenemylist_2
        (`/Engine/EditorBlueprintResources/StandardMacros.IsValid` _array_element
          (:`Is Not Valid`
            (`KismetArrayLibrary.Array_RemoveItem` _spawnedenemylist_2 _array_element))))
      (if (and (<= (`self.tempTime`) 0.0) (< (`KismetArrayLibrary.Array_Length` (`self.SpawnedEnemyList`)) (`self.MaxTimeSpawn`)))
        (if (> (`self.tempTimeSpawnNumber`) 0) :!label _label
          (bind _keys (`BlueprintMapLibrary.Map_Keys` (`self.EnemyList`)))
          (`self.RandomSpawn`)
          (bind _outitem (`KismetArrayLibrary.Array_Random` _keys))
          (bind _asenemy_bp (castclass `/Game/Blueprints/Enemy/Enemy_BP` _outitem))
          (switch `/Game/Blueprints/Enemy/Enemy_Type_Enum` (`.EnemyType` (defaults `Object` _asenemy_bp))
            (:`NewEnumerator0`
              (bind _returnvalue (`AIBlueprintHelperLibrary.SpawnAIFromClass` _outitem "/Game/AI/OldAI/RangeEnemy_AI_BT.RangeEnemy_AI_BT" _tempspawnpoint (struct) false null))
              (`KismetArrayLibrary.Array_Add` (`self.SpawnedEnemyList`) _returnvalue))
            (:`NewEnumerator1`
              (bind _returnvalue_2 (`AIBlueprintHelperLibrary.SpawnAIFromClass` _outitem "/Game/AI/OldAI/CloseCombatEnemy_AI_BT.CloseCombatEnemy_AI_BT" _tempspawnpoint (struct) false null))
              (`KismetArrayLibrary.Array_Add` (`self.SpawnedEnemyList`) _returnvalue_2)))
          (set `self.tempTimeSpawnNumber` (- (`self.tempTimeSpawnNumber`) 1))
          (goto _label)
          (else
            (set `self.tempTimeSpawnNumber` (`self.TimeSpawnNumber`))
            (set `self.tempTime` (`self.SpwanTime`))))
        (else
          (set `self.tempTime` (- (`self.tempTime`) (`GameplayStatics.GetWorldDeltaSeconds`))))))
    (:`NewEnumerator1`
      (for _array_element_2 _spawnedenemylist
        (`/Engine/EditorBlueprintResources/StandardMacros.IsValid` _array_element_2
          (:`Is Not Valid`
            (`KismetArrayLibrary.Array_RemoveItem` _spawnedenemylist _array_element_2))))
      (if (<= (`KismetArrayLibrary.Array_Length` _spawnedenemylist) 0)
        (`self.SpawnEnemy`)))))

(fn `RandomSpawn`
  (set `self.tempSpawnPoint` (+ (`self.SpawnPoint`) (`KismetMathLibrary.MakeVector` (`KismetMathLibrary.RandomFloatInRange` -250.0 250.0) (`KismetMathLibrary.RandomFloatInRange` -250.0 250.0)))))

(fn `SpawnEnemy`
  (bind _tempspawnpoint (`self.tempSpawnPoint`))
  (bind _enemylist (`self.EnemyList`))
  (bind _keys (`BlueprintMapLibrary.Map_Keys` _enemylist))
  (for _array_element _keys
    (set `self.tempSpawnNumber` (`BlueprintMapLibrary.Map_Find` _enemylist _array_element))
    (`self.RandomSpawn` :!label _label)
    (bind _asenemy_bp (castclass `/Game/Blueprints/Enemy/Enemy_BP` _array_element))
    (switch `/Game/Blueprints/Enemy/Enemy_Type_Enum` (`.EnemyType` (defaults `Object` _asenemy_bp))
      (:`NewEnumerator0`
        (bind _returnvalue (`AIBlueprintHelperLibrary.SpawnAIFromClass` _array_element "/Game/AI/OldAI/RangeEnemy_AI_BT.RangeEnemy_AI_BT" _tempspawnpoint (struct) false null))
        (`KismetArrayLibrary.Array_Add` (`self.SpawnedEnemyList`) _returnvalue))
      (:`NewEnumerator1`
        (bind _returnvalue_2 (`AIBlueprintHelperLibrary.SpawnAIFromClass` _array_element "/Game/AI/OldAI/CloseCombatEnemy_AI_BT.CloseCombatEnemy_AI_BT" _tempspawnpoint (struct) false null))
        (`KismetArrayLibrary.Array_Add` (`self.SpawnedEnemyList`) _returnvalue_2)))
    (if (> (`self.tempSpawnNumber`) 1)
      (set `self.tempSpawnNumber` (- (`self.tempSpawnNumber`) 1))
      (goto _label))))

(fn `UserConstructionScript`)