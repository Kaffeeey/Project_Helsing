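; Enemy manager that decides which enemies may attack the player, capping simultaneous attackers per enemy type.
; Every ninth tick it removes invalid and duplicate entries from EnemyList and splits it into range, close combat, boss and flying range lists.
; For each list it maps indices to player distance, sorts nearest first, and grants AllowedToAttack to the closest enemies that see the player, revoking it once the limit fills.
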(event `self.ReceiveBeginPlay`
  (set `self.Player` (`GameplayStatics.GetPlayerPawn` 0)))

(event `self.ReceiveTick`
  (params (DeltaSeconds :type "Float (single-precision)"))
  (if (> (`self.FixedUpdateCount`) 0)
    (set `self.FixedUpdateCount` (- (`self.FixedUpdateCount`) 1))
    (else
      (`self.FixedUpdate`)
      (set `self.FixedUpdateCount` 8))))

(event `FixedUpdate`
  (bind _enemyoutlist (`self.ClearDoubleEnemys` (`self.EnemyList`)))
  (`self.SortByEnemyType` _enemyoutlist)
  (bind _enemydistancelist (`self.CreateDistanceList` (`self.RangeEnemyList`)))
  (bind _enemydistanceoutlist (`self.SortListByLength` _enemydistancelist))
  (`self.SetEnemyFightingOrder` _enemydistanceoutlist (`self.RangeEnemyList`) (`self.NumberOfRangeEnemiesToAttack`))
  (bind _enemydistancelist_2 (`self.CreateDistanceList` (`self.CloseCombatEnemyList`)))
  (bind _enemydistanceoutlist_2 (`self.SortListByLength` _enemydistancelist_2))
  (`self.SetEnemyFightingOrder` _enemydistanceoutlist_2 (`self.CloseCombatEnemyList`) (`self.NumberOfCloseCombarEnemiesToAttack`))
  (bind _enemydistancelist_3 (`self.CreateDistanceList` (`self.BossEnemyList`)))
  (bind _enemydistanceoutlist_3 (`self.SortListByLength` _enemydistancelist_3))
  (`self.SetEnemyFightingOrder` _enemydistanceoutlist_3 (`self.BossEnemyList`) (`self.NumberOfBossEnemiesToAttack`))
  (bind _enemydistancelist_4 (`self.CreateDistanceList` (`self.FlyingRangeEnemyList`)))
  (bind _enemydistanceoutlist_4 (`self.SortListByLength` _enemydistancelist_4))
  (`self.SetEnemyFightingOrder` _enemydistanceoutlist_4 (`self.FlyingRangeEnemyList`) (`self.NumberOfFlyingRangeEnemyToAttack`)))

(fn `ClearDoubleEnemys`
  (params (EnemyInList :type "Array of /Game/Blueprints/Enemy/BP_Enemy Object Reference"))
  (returns (EnemyOutList :type "Array of /Game/Blueprints/Enemy/BP_Enemy Object Reference"))
  (locals (UnsortedList :type "Array of /Game/Blueprints/Enemy/BP_Enemy Object Reference") (SortedList :type "Array of /Game/Blueprints/Enemy/BP_Enemy Object Reference"))
  (bind _output_get (set `local.UnsortedList` EnemyInList))
  (for _array_element _output_get
    (`/Engine/EditorBlueprintResources/StandardMacros.IsValid` _array_element
      (:`Is Valid`
        (`KismetArrayLibrary.Array_AddUnique` (`local.SortedList`) _array_element))))
  (return (`local.SortedList`)))

(fn `CreateDistanceList`
  (params (EnemyList :type "Array of /Game/Blueprints/Enemy/BP_Enemy Object Reference"))
  (returns (EnemyDistanceList :type "Map of Integer to Float (double-precision)"))
  (locals (EnemyDistanceLocalList :type "Map of Integer to Float (double-precision)") (EnemyLocalList :type "Array of /Game/Blueprints/Enemy/BP_Enemy Object Reference"))
  (bind _output_get (set `local.EnemyLocalList` EnemyList))
  (for (_array_element _array_index) _output_get
    (if (`KismetSystemLibrary.IsValid` _array_element)
      (`BlueprintMapLibrary.Map_Add` (`local.EnemyDistanceLocalList`) _array_index (`KismetMathLibrary.Vector_Distance` (`self.K2_GetActorLocation` _array_element) (`self.K2_GetActorLocation` (`self.Player`))))
      (else
        (`KismetArrayLibrary.Array_RemoveItem` (`local.EnemyLocalList`) _array_element))))
  (return (`local.EnemyDistanceLocalList`)))

(fn `FindKey`
  (params (MapIn :type "Map of Integer to Float (double-precision)") (ValueIn :type "Float (double-precision)"))
  (returns (KeyOut :type Integer))
  (locals (TempMap :type "Map of Integer to Float (double-precision)"))
  (bind _output_get (set `local.TempMap` MapIn))
  (bind _keys (`BlueprintMapLibrary.Map_Keys` _output_get))
  (for _array_element _keys
    (if (== ValueIn (`BlueprintMapLibrary.Map_Find` (`local.TempMap`) _array_element))
      (return _array_element))))

(fn `SetEnemyFightingOrder`
  (params (EnemyDistanceList :type "Map of Integer to Float (double-precision)") (EnemyList :type "Array of /Game/Blueprints/Enemy/BP_Enemy Object Reference") (NumberOfFightingEnemy :type Integer))
  (locals (TempEnemyDistanceList :type "Map of Integer to Float (double-precision)") (TempEnemyList :type "Array of /Game/Blueprints/Enemy/BP_Enemy Object Reference") (TmpNumberOfFightingEnemy :type Integer) (TempIndexNumber :type Integer :default 0))
  (set `local.TempEnemyDistanceList` EnemyDistanceList)
  (set `local.TempEnemyList` EnemyList)
  (set `local.TmpNumberOfFightingEnemy` NumberOfFightingEnemy)
  (bind _values (`BlueprintMapLibrary.Map_Values` (`local.TempEnemyDistanceList`)))
  (for _array_element _values
    (if (< (`local.TempIndexNumber`) (`local.TmpNumberOfFightingEnemy`))
      (bind _keyout (`self.FindKey` (`local.TempEnemyDistanceList`) _array_element))
      (bind _output (`|GetArrayItem` (`local.TempEnemyList`) _keyout))
      (if (`/Game/Blueprints/Enemy/BP_Enemy.CanSeePlayer` _output)
        (set `/Game/Blueprints/Enemy/BP_Enemy.AllowedToAttack` true _output)
        (set `local.TempIndexNumber` (+ (`local.TempIndexNumber`) 1)))
      (else
        (bind _keyout_2 (`self.FindKey` (`local.TempEnemyDistanceList`) _array_element))
        (set `/Game/Blueprints/Enemy/BP_Enemy.AllowedToAttack` false (`|GetArrayItem` (`local.TempEnemyList`) _keyout_2))))))

(fn `SortByEnemyType`
  (params (SortListIn :type "Array of /Game/Blueprints/Enemy/BP_Enemy Object Reference"))
  (locals (UnsortedList :type "Array of /Game/Blueprints/Enemy/BP_Enemy Object Reference"))
  (set `local.UnsortedList` SortListIn)
  (`KismetArrayLibrary.Array_Clear` (`self.RangeEnemyList`))
  (`KismetArrayLibrary.Array_Clear` (`self.CloseCombatEnemyList`))
  (`KismetArrayLibrary.Array_Clear` (`self.BossEnemyList`))
  (`KismetArrayLibrary.Array_Clear` (`self.FlyingRangeEnemyList`))
  (for _array_element (`local.UnsortedList`)
    (switch `/Game/Blueprints/Enemy/Enum_Enemy_Type` (`/Game/Blueprints/Enemy/BP_Enemy.EnemyType` _array_element)
      (:`NewEnumerator0`
        (`KismetArrayLibrary.Array_Add` (`self.RangeEnemyList`) _array_element))
      (:`NewEnumerator1`
        (`KismetArrayLibrary.Array_Add` (`self.CloseCombatEnemyList`)))
      (:`NewEnumerator2`
        (`KismetArrayLibrary.Array_Add` (`self.BossEnemyList`)))
      (:`NewEnumerator3`
        (`KismetArrayLibrary.Array_Add` (`self.FlyingRangeEnemyList`))))))

(fn `SortListByLength`
  (params (EnemyDistanceInList :type "Map of Integer to Float (double-precision)"))
  (returns (EnemyDistanceOutList :type "Map of Integer to Float (double-precision)"))
  (locals (TempEnemyDistanceInList :type "Map of Integer to Float (double-precision)") (Sorted_List :type "Array of Float (double-precision)") (TempEnemyDistanceOutList :type "Map of Integer to Float (double-precision)"))
  (bind _output_get (set `local.TempEnemyDistanceInList` EnemyDistanceInList))
  (bind _values (`BlueprintMapLibrary.Map_Values` _output_get))
  (bind _outarray (`/Game/AI/FunctionLibrary_AI.SortFloatArrayMinToMax` _values))
  (for _array_element _outarray
    (bind _keys (`BlueprintMapLibrary.Map_Keys` (`local.TempEnemyDistanceInList`)))
    (for _array_element_2 _keys
      (if (== _array_element (`BlueprintMapLibrary.Map_Find` (`local.TempEnemyDistanceInList`) _array_element_2))
        (`BlueprintMapLibrary.Map_Add` (`local.TempEnemyDistanceOutList`) _array_element_2 _array_element)
        (break))))
  (return (`local.TempEnemyDistanceOutList`)))

(fn `UserConstructionScript`)