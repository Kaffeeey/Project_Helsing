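; Flying ranged enemy that feeds player-proximity state to its AI controller's blackboard.
; Each FixedUpdate it runs sphere overlaps for the player character at FightingRange and PersonalSpace radii, writing PlayerInRange and PlayerInPersonalSpace keys.
; It also sets AwakeRange true when AIFightingDistance is within AwakeTriggerRange, and never clears it here.
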(event `self.ReceiveTick`
  (params (DeltaSeconds :type "Float (single-precision)"))
  (`parent.ReceiveTick` DeltaSeconds))

(event `self.FixedUpdate`
  (bind _returnvalue (`AIBlueprintHelperLibrary.GetAIController` self))
  (`parent.FixedUpdate`)
  (bind _playercheck (`self.DistanceCheck` (`self.FightingRange`)))
  (set `self.PlayerInRange` _playercheck)
  (bind _playercheck_2 (`self.DistanceCheck` (`self.PersonalSpace`)))
  (set `self.PlayerInPersonalSpace` _playercheck_2)
  (`/Game/AI/FunctionLibrary_AI.Set_BB_Key` "NewEnumerator0" _returnvalue "PlayerInRange" (`self.PlayerInRange`))
  (`/Game/AI/FunctionLibrary_AI.Set_BB_Key` "NewEnumerator0" _returnvalue "PlayerInPersonalSpace" (`self.PlayerInPersonalSpace`))
  (if (not (> (`self.AIFightingDistance`) (`self.AwakeTriggerRange`)))
    (`/Game/AI/FunctionLibrary_AI.Set_BB_Key` "NewEnumerator0" _returnvalue "AwakeRange" true)))

(fn `DistanceCheck`
  (params (Distance :type "Float (double-precision)"))
  (returns (PlayerCheck :type Boolean))
  (bind _outactors (`KismetSystemLibrary.SphereOverlapActors` (`self.K2_GetActorLocation` self) Distance (`self.Object Types`) "/Game/Blueprints/FPSChar_V_0_3.FPSChar_V_0_3_C"))
  (for _array_element _outactors
    (cast `/Game/Blueprints/FPSChar_V_0_3` _array_element)
    (return true))
  (return false))

(fn `UserConstructionScript`
  (`parent.UserConstructionScript`))