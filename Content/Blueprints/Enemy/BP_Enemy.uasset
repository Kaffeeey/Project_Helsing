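; Base enemy character for the FPS, with ranged, melee and flying ranged types chosen by EnemyType.
; Every eighth tick it aims at the player and feeds distance, type and cooldown to the AI blackboard; an EQS event picks move targets.
; Damage scales by bone hit zone and crit, with weakpoint hits paralyzing the enemy on a timer.
; Death ragdolls the mesh, rolls item and money drops, then destroys the corpse.
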(event `FixedUpdate`
  (`self.SetAIVariables`)
  (`SceneComponent.K2_SetWorldRotation` (`self.BulletPoint`) (`KismetMathLibrary.MakeRotFromX` (`KismetMathLibrary.GetDirectionUnitVector` (`SceneComponent.K2_GetComponentLocation` (`self.BulletPoint`)) (`self.K2_GetActorLocation` (`GameplayStatics.GetPlayerPawn` 0)))) false false)
  (`TextRenderComponent.K2_SetText` (`self.DevParalyze`) (`KismetTextLibrary.Conv_DoubleToText` (`self.Paralyze Time`) "HalfToEven"))
  (`TextRenderComponent.K2_SetText` (`self.DevHP`) (`KismetTextLibrary.Conv_DoubleToText` (`self.HP`) "HalfToEven")))

(event `self.ReceiveBeginPlay`
  (set `CharacterMovementComponent.MaxWalkSpeed` (`self.Speed`) (`self.CharacterMovement`)))

(event `StartAttacking`
  (`self.Attack`))

(event `StopAttacking`)

(event `self.ReceiveTick`
  (params (DeltaSeconds :type "Float (single-precision)"))
  (if (not (`self.Dead`))
    (`self.PlayRandomSFX` (`SceneComponent.K2_GetComponentLocation` (`self.Mesh`)) DeltaSeconds)
    ;[1 1 1] FixedUpdate
    (set `self.FixedUpdateCount` (+ (`self.FixedUpdateCount`) 1))
    (if (>= (`self.FixedUpdateCount`) 8)
      (`self.FixedUpdate`)
      (set `self.FixedUpdateCount` 0))
    (if (`self.Paralyzed`)
      (if (> (`self.Paralyze Time`) 0.0)
        (set `self.Paralyze Time` (- (`self.Paralyze Time`) (`GameplayStatics.GetWorldDeltaSeconds`)))
        (else
          (set `self.Paralyzed` false)
          (`/Game/AI/FunctionLibrary_AI.Set_BB_Key` "NewEnumerator0" (`AIBlueprintHelperLibrary.GetAIController` self) "Paralyzed_AI" (`self.Paralyzed`)))))))

(event `RunEQS`
  (bind _returnvalue (`EnvQueryManager.RunEQSQuery` "/Game/AI/OldAI/EQS_Enemy_AI.EQS_Enemy_AI" null "SingleResult" "/Script/AIModule.EnvQueryInstanceBlueprintWrapper"))
  (bind _resultlocations (`EnvQueryInstanceBlueprintWrapper.GetQueryResultsAsLocations` _returnvalue))
  (for (_array_element _array_index) _resultlocations
    (if (== _array_index 0)
      (set `self.Temp Dis 1` (`KismetMathLibrary.Vector_Distance` _array_element (`self.K2_GetActorLocation` self)))
      (set `self.Temp Dis 2` (`KismetMathLibrary.Vector_Distance` _array_element (`self.K2_GetActorLocation` (`GameplayStatics.GetPlayerPawn` 0))))
      (set `self.Temp Target Pos` _array_element)
      (elif (and (< (`KismetMathLibrary.Vector_Distance` (`self.K2_GetActorLocation` (`GameplayStatics.GetPlayerPawn` 0)) _array_element) (`self.Temp Dis 2`)) (< (`KismetMathLibrary.Vector_Distance` (`self.K2_GetActorLocation` self) _array_element) (`self.Temp Dis 1`)))
        (set `self.Temp Target Pos` _array_element))))
  (`BlackboardComponent.SetValueAsVector` (`AIBlueprintHelperLibrary.GetBlackboard` (`AIBlueprintHelperLibrary.GetAIController` self)) "TargetLocation" (`self.Temp Target Pos`)))

(event `Wiggle`
  (params (Bone :type Name))
  (bind _mesh (`self.Mesh`))
  (`SkeletalMeshComponent.SetAllBodiesBelowSimulatePhysics` _mesh Bone true true)
  (`SkeletalMeshComponent.SetAllBodiesBelowPhysicsBlendWeight` _mesh Bone 1.0 false true)
  (`KismetSystemLibrary.Delay` 0.5)
  (`SkeletalMeshComponent.SetAllBodiesBelowPhysicsBlendWeight` _mesh Bone 0.0 false true))

(event `DeleteEnemyCorpse`
  (`KismetSystemLibrary.Delay` 5.0)
  (`self.K2_DestroyActor`))

(fn `Attack`
  (switch `/Game/Blueprints/Enemy/Enum_Enemy_Type` (`self.EnemyType`)
    (:`NewEnumerator0`
      (`self.FireBullet` "/Game/Blueprints/Enemy/BP_Fast_Smal_Enemy_Projectile.BP_Fast_Smal_Enemy_Projectile_C"))
    (:`NewEnumerator1`
      (`self.CloseCombatAttack`))
    (:`NewEnumerator3`
      (`self.FireBullet` "/Game/Blueprints/Enemy/BP_Slow_Big_Enemy_Projectile.BP_Slow_Big_Enemy_Projectile_C"))))

(fn `CloseCombatAttack`
  (locals (HitObjectTypes :type "Array of EObjectTypeQuery Enum"))
  (bind _capsulecomponent (`self.CapsuleComponent`))
  (if (`self.CanFire`)
    (bind _outactors (`KismetSystemLibrary.SphereOverlapActors` (+ (`SceneComponent.K2_GetComponentLocation` _capsulecomponent) (* (`SceneComponent.GetForwardVector` _capsulecomponent) 1.0)) 100.0 (`local.HitObjectTypes`) "/Game/Blueprints/FPSChar_V_0_3.FPSChar_V_0_3_C"))
    (for _array_element _outactors
      (bind _asfpschar_v_0_3 (cast `/Game/Blueprints/FPSChar_V_0_3` _array_element))
      (`/Game/Blueprints/FPSChar_V_0_3.TakeDamage` _asfpschar_v_0_3 (`self.MonsterDMG`))
      (set `self.CanFire` false))))

(fn `Death`
  (params (RNGesus :type "Float (double-precision)") (MoneyChance :type "Float (double-precision)") (MoneyMultiply :type "Float (double-precision)"))
  (bind _mesh (`self.Mesh`))
  (bind _returnvalue (`SkinnedMeshComponent.GetBoneName` (`self.Mesh`) 0))
  (bind _returnvalue_location (`KismetMathLibrary.BreakTransform` (`self.GetTransform` self)))
  (bind _hit (`self.Random` RNGesus))
  (if _hit
    (`|SpawnActorFromClass` "/Game/Blueprints/WeightedPicker/ItemSpawn.ItemSpawn_C" (`KismetMathLibrary.MakeTransform` _returnvalue_location) "Undefined" "OverrideRootScale" null null))
  (bind _hit_2 (`self.Random` MoneyChance))
  (if _hit_2
    (`self.GiveMoney` MoneyMultiply))
  (if (!= _returnvalue "None")
    (`PrimitiveComponent.SetCollisionResponseToChannel` _mesh "ECC_Pawn" "ECR_Ignore")
    (`PrimitiveComponent.SetCollisionResponseToChannel` _mesh "ECC_GameTraceChannel2" "ECR_Ignore")
    (`SkeletalMeshComponent.SetAllBodiesBelowSimulatePhysics` _mesh _returnvalue true true)
    (`SkeletalMeshComponent.SetAllBodiesBelowPhysicsBlendWeight` _mesh _returnvalue 0.9 false true))
  (`self.DeleteEnemyCorpse`))

(fn `DebugMode`
  (bind _output_get (set `self.Debug` (!= (`self.Debug`) true)))
  (`SceneComponent.SetVisibility` (`self.DevHP`) _output_get false)
  (`SceneComponent.SetVisibility` (`self.DevParalyze`) _output_get false))

(fn `FireBullet`
  (params (Projectile :type "Actor Class Reference"))
  (bind _returnvalue (`|SpawnActorFromClass` Projectile (`KismetMathLibrary.MakeTransform` (`SceneComponent.K2_GetComponentLocation` (`self.BulletPoint`)) (`KismetMathLibrary.Quat_Rotator` (`KismetMathLibrary.Conv_VectorToQuaternion` (`SceneComponent.GetForwardVector` (`self.BulletPoint`))))) "Undefined" "OverrideRootScale" null null))
  (bind _asbp_enemy_projectile (cast `/Game/Blueprints/Enemy/BP_Enemy_Projectile` _returnvalue))
  (set `/Game/Blueprints/Enemy/BP_Enemy_Projectile.Damage` (`self.MonsterDMG`) _asbp_enemy_projectile))

(fn `GetDamage`
  (params (Damage :type "Float (double-precision)") (ParalyzeTime :type "Float (double-precision)" :default 1.0) (CritMultiplier :type "Float (double-precision)") (RNGesus :type "Float (double-precision)" :default 0.0) (MoneyChance :type "Float (double-precision)") (MoneyMultiply :type "Float (double-precision)") (Crit :type Boolean) (HitBoneName :type Name) (HitPosition :type "Vector Structure") (HitDirection :type "Rotator Structure") (DamageType :type "/Game/Blueprints/Enemy/Enum_DMG_Type Enum" :default "NewEnumerator0"))
  (returns (kill :type Boolean))
  (locals (IncomingDMG :type "Float (double-precision)"))
  (bind _output_get (set `local.IncomingDMG` Damage))
  ;[1 1 1] DMG Type Switch
  (switch `/Game/Blueprints/Enemy/Enum_DMG_Type` DamageType
    (:`NewEnumerator1`
      _)
    (:`NewEnumerator0`
      ;[1 1 1] HitBox Detection
      (bind _dmgmultiplier (`self.HitBox` HitBoneName ParalyzeTime))
      (bind _output_get_2 (set `local.IncomingDMG` (* _output_get _dmgmultiplier)))))
  (if (> _output_get_2 0.0)
    (`|SpawnActorFromClass` (`self.BloodDecal`) (`KismetMathLibrary.MakeTransform` HitPosition HitDirection) "Undefined" "OverrideRootScale" null null)
    (if Crit
      (set `local.IncomingDMG` (* (`local.IncomingDMG`) CritMultiplier)))
    ;[1 1 1] DMG Calculation
    (bind _output_get_3 (set `self.HP` (- (`self.HP`) (`local.IncomingDMG`))))
    (bind _returnvalue (<= _output_get_3 0.0))
    ;[1 1 1] Enemy Death
    (if _returnvalue
      (set `self.Dead` _returnvalue)
      (`/Game/AI/FunctionLibrary_AI.Set_BB_Key` "NewEnumerator0" (`AIBlueprintHelperLibrary.GetAIController` self) "Dead" (`self.Dead`))
      (`self.Death` RNGesus MoneyChance MoneyMultiply))
    (return (`self.Dead`))))

(fn `GiveMoney`
  (params (MoneyMultiply :type "Float (double-precision)"))
  (bind _asfpschar_v_0_3 (cast `/Game/Blueprints/FPSChar_V_0_3` (`GameplayStatics.GetPlayerPawn` 0)))
  (set `/Game/Blueprints/FPSChar_V_0_3.Currency` (+ (`/Game/Blueprints/FPSChar_V_0_3.Currency` _asfpschar_v_0_3) (`KismetMathLibrary.FTrunc` (* (`self.MoneyDrop`) MoneyMultiply))) _asfpschar_v_0_3))

(fn `HitBox`
  (params (HitBone :type Name) (ParalyzeTime :type "Float (double-precision)"))
  (returns (DMGMultiplier :type "Float (double-precision)"))
  (if (!= HitBone "None")
    (if (and (== (`KismetArrayLibrary.Array_Length` (`self.HeadBones`)) 0) (== (`KismetArrayLibrary.Array_Length` (`self.TorsoBones`)) 0) (== (`KismetArrayLibrary.Array_Length` (`self.LimbBones`)) 0) (== (`KismetArrayLibrary.Array_Length` (`self.WeakpointBones`)) 0))
      (return 1.0)
      (else
        (for _array_element (`self.HeadBones`)
          (if (== _array_element HitBone)
            (bind _output_get (set `self.DMGMultiplier` (`self.HeadDMGMultiply`)))
            (return _output_get)))
        (for _array_element_2 (`self.TorsoBones`)
          (if (== _array_element_2 HitBone)
            (bind _output_get_2 (set `self.DMGMultiplier` (`self.TorsoDMGMultipy`)))
            (return _output_get_2)))
        (for _array_element_3 (`self.LimbBones`)
          (if (== _array_element_3 HitBone)
            (bind _output_get_3 (set `self.DMGMultiplier` (`self.LimbDMGMultiply`)))
            (return _output_get_3)))
        (for _array_element_4 (`self.WeakpointBones`)
          (if (== _array_element_4 HitBone)
            (`self.Paralyze` ParalyzeTime)
            (bind _output_get_4 (set `self.DMGMultiplier` (`self.WeakpointDMGMultiply`)))
            (return _output_get_4)))))
    (else
      (return 1.0))))

(fn `Paralyze`
  (params (ParalyzeTime :type "Float (double-precision)"))
  (set `self.Paralyze Time` ParalyzeTime)
  (set `self.Paralyzed` true)
  (`/Game/AI/FunctionLibrary_AI.Set_BB_Key` "NewEnumerator0" (`AIBlueprintHelperLibrary.GetAIController` self) "Paralyzed_AI" (`self.Paralyzed`)))

(fn `PlayRandomSFX`
  (params (SoundPosition :type "Vector Structure") (Second :type "Float (double-precision)"))
  (bind _outitem (`KismetArrayLibrary.Array_Random` (`self.MonsterSound`)))
  (if (> (`KismetArrayLibrary.Array_Length` (`self.MonsterSound`)) 0)
    (if (`KismetMathLibrary.RandomBool`)
      (if (<= (`self.CurrentSoundLength`) 0.0)
        (set `self.CurrentSoundLength` (+ (`SoundBase.Duration` _outitem) 3.0))
        (`GameplayStatics.PlaySoundAtLocation` _outitem SoundPosition (struct) 1.0 1.0 0.0 null null null)
        (else
          (set `self.CurrentSoundLength` (- (`self.CurrentSoundLength`) Second)))))))

(fn `Random`
  (params (RandomParam :type "Float (double-precision)"))
  (returns (hit :type Boolean))
  (return (<= (`KismetMathLibrary.RandomFloatInRange` 0.0 1.0) (`KismetMathLibrary.FClamp` RandomParam))))

(fn `SetAIVariables`
  (bind _returnvalue (`AIBlueprintHelperLibrary.GetAIController` self))
  (`/Game/AI/FunctionLibrary_AI.Set_BB_Key` "NewEnumerator3" _returnvalue "FightDistance" false null 0 (`KismetMathLibrary.Vector_Distance` (`self.K2_GetActorLocation` self) (`self.K2_GetActorLocation` (`GameplayStatics.GetPlayerCharacter` 0))))
  (`/Game/AI/FunctionLibrary_AI.Set_BB_Key` "NewEnumerator2" _returnvalue "EnemyType" false null (`self.EnemyType`))
  (`/Game/AI/FunctionLibrary_AI.Set_BB_Key` "NewEnumerator2" _returnvalue "TestMode" false null (`self.TestMode`))
  (`/Game/AI/FunctionLibrary_AI.Set_BB_Key` "NewEnumerator3" _returnvalue "FireCooldown" false null 0 (`self.FireRate`)))

(fn `UserConstructionScript`)