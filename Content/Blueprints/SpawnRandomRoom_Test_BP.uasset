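; SpawnRandomRoom_Test_BP is a test Blueprint that streams in a randomly chosen room level when an actor begins overlapping it.
; If RoomList has entries, it looks one up by a random integer and passes its name to LoadLevelInstance at RoomPosition and RoomRotation.
; The returned level instance is stored in Test, and the overlap has no actor filter or one-shot guard.
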(event `self.ReceiveActorBeginOverlap`
  (params (OtherActor :type "Actor Object Reference"))
  (bind _returnvalue (`BlueprintMapLibrary.Map_Length` (`self.RoomList`)))
  (if (> _returnvalue 0)
    (bind (_boutsuccess _returnvalue_2) (`LevelStreamingDynamic.LoadLevelInstance` (`KismetStringLibrary.Conv_NameToString` (`BlueprintMapLibrary.Map_Find` (`self.RoomList`) (`KismetMathLibrary.RandomIntegerInRange` 0 (- _returnvalue 1)))) (`self.RoomPosition`) (`self.RoomRotation`)))
    (set `self.test` _returnvalue_2)))

(fn `UserConstructionScript`)