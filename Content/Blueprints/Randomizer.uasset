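; Randomizer actor that scatters a set number of blood tanks and hook points across the level's spawn points on BeginPlay.
; Two sequential loops gather all spawn point actors of each type and reshuffle them every iteration.
; A shared random chance roll either spawns at the current index and decrements the remaining count, or advances the index.
; Chosen points are not excluded from later picks here.
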(event `self.ReceiveBeginPlay`
  (while (> (`self.BloodTankSpawnCount`) 0)
    (bind _outactors (`GameplayStatics.GetAllActorsOfClass` "/Game/Blueprints/BloodTankSpawnPoint.BloodTankSpawnPoint_C"))
    (`KismetArrayLibrary.Array_Shuffle` _outactors)
    (if (> (`self.SpawnChance`) (`KismetMathLibrary.RandomFloat`))
      (`/Game/Blueprints/BloodTankSpawnPoint.SpawnBloodtank` (`|GetArrayItem` _outactors (`self.Index`)))
      (set `self.Index` 0)
      (`/Engine/EditorBlueprintResources/StandardMacros.DecrementInt` (`self.BloodTankSpawnCount`))
      (elif (> (`self.Index`) (`KismetArrayLibrary.Array_Length` _outactors))
        (set `self.Index` 0)
        (else
          (`/Engine/EditorBlueprintResources/StandardMacros.IncrementInt` (`self.Index`))))))
  (set `self.Index` 0)
  (while (> (`self.HookPointSpawnCount`) 0)
    (bind _outactors_2 (`GameplayStatics.GetAllActorsOfClass` "/Game/Blueprints/HookPointSpawnPoint.HookPointSpawnPoint_C"))
    (`KismetArrayLibrary.Array_Shuffle` _outactors_2)
    (if (> (`self.SpawnChance`) (`KismetMathLibrary.RandomFloat`))
      (`/Game/Blueprints/HookPointSpawnPoint.SpawnHookPoint` (`|GetArrayItem` _outactors_2 (`self.Index`)))
      (set `self.Index` 0)
      (`/Engine/EditorBlueprintResources/StandardMacros.DecrementInt` (`self.HookPointSpawnCount`))
      (elif (> (`self.Index`) (`KismetArrayLibrary.Array_Length` _outactors_2))
        (set `self.Index` 0)
        (else
          (`/Engine/EditorBlueprintResources/StandardMacros.IncrementInt` (`self.Index`)))))))

(fn `UserConstructionScript`)