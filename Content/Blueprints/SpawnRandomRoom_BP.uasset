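; Trigger actor that streams in a random room level when any actor begins overlapping it.
; On overlap it calls UnloadLevel on each entry in UnloadLevelList, then loads a random Level entry as an instance at RoomPosition and RoomRotation.
; The instance takes UnloadLevelName as its name override, which UnloadLevel uses to unload that level before destroying the actor.
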(event `self.ReceiveActorBeginOverlap`
  (params (OtherActor :type "Actor Object Reference"))
  (if (> (`KismetArrayLibrary.Array_Length` (`self.UnloadLevelList`)) 0)
    (`self.UnloadLevelFromList`))
  (if (> (`KismetArrayLibrary.Array_Length` (`self.Level`)) 0)
    (`LevelStreamingDynamic.LoadLevelInstanceBySoftObjectPtr` (`KismetArrayLibrary.Array_Random` (`self.Level`)) (`self.RoomPosition`) (`self.RoomRotation`) (`self.UnloadLevelName`))))

(event `UnloadLevel`
  (`GameplayStatics.UnloadStreamLevel` (`KismetStringLibrary.Conv_StringToName` (`self.UnloadLevelName`)))
  (`self.K2_DestroyActor`))

(event `UnloadLevelFromList`
  (bind _unloadlevellist (`self.UnloadLevelList`))
  (if (> (`KismetArrayLibrary.Array_Length` _unloadlevellist) 0)
    (for _array_element _unloadlevellist
      (`self.UnloadLevel` _array_element))))

(fn `UserConstructionScript`)