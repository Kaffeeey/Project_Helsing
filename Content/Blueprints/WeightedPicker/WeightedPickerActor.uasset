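; WeightedPickerActor picks a random entry from its WeightedItems map, using weights read from each entry's class defaults.
; Pick calls GetMaxWeight to add all weights onto MaxWeight, then PickItem draws a truncated random threshold within that total.
; PickItem counts MaxWeight down through each item's weight span and returns the item where it meets the threshold.
; MaxWeight doubles as the countdown and is never explicitly reset between picks.
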(fn `GetMaxWeight`
  (bind _values (`BlueprintMapLibrary.Map_Values` (`self.WeightedItems`)))
  (for _array_element _values
    (set `self.MaxWeight` (+ (defaults `Object` _array_element) (`self.MaxWeight`)))))

(fn `Pick`
  (returns (Pick :type "/Game/Blueprints/WeightedPicker/WeightedItem Class Reference"))
  (`self.GetMaxWeight`)
  (bind _item (`self.PickItem`))
  (return _item))

(fn `PickItem`
  (returns (Item :type "/Game/Blueprints/WeightedPicker/WeightedItem Class Reference"))
  (set `self.Weight` (`KismetMathLibrary.FTrunc` (* (`self.MaxWeight`) (`KismetMathLibrary.RandomFloatInRange` 0.0 1.0))))
  (bind _values (`BlueprintMapLibrary.Map_Values` (`self.WeightedItems`)))
  (for _array_element _values
    (for _ (range (+ (defaults `Object` _array_element) 1))
      (if (== (`self.MaxWeight`) (`self.Weight`))
        (return _array_element)
        (else
          (bind _result (`/Engine/EditorBlueprintResources/StandardMacros.DecrementInt` (`self.MaxWeight`))
            (:`  `
              (set `self.MaxWeight` _result))))))))

(fn `UserConstructionScript`)