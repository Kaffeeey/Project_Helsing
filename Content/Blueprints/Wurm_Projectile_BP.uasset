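; Wurm projectile Blueprint that damages the FPSChar it hits.
; The Hit event casts the other actor to FPSChar and subtracts Damage directly from its HP.
; The DestroyActor branch follows an equality check that always passes after a successful cast, and a failed cast stops execution, so the projectile never destroys itself here.
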(event `self.ReceiveBeginPlay`)

(event `self.ReceiveTick`
  (params (DeltaSeconds :type "Float (single-precision)")))

(event `self.ReceiveHit`
  (params (MyComp :type "PrimitiveComponent Object Reference") (Other :type "Actor Object Reference") (OtherComp :type "PrimitiveComponent Object Reference") (bSelfMoved :type Boolean) (HitLocation :type "Vector Structure") (HitNormal :type "Vector Structure") (NormalImpulse :type "Vector Structure") (Hit :type "HitResult Structure (by ref)"))
  (bind _asfpschar (cast `/Game/Blueprints/FPSChar` Other))
  (if (== Other _asfpschar)
    (bind _asfpschar_2 (cast `/Game/Blueprints/FPSChar` Other))
    (set `/Game/Blueprints/FPSChar.HP` (- (`/Game/Blueprints/FPSChar.HP` _asfpschar_2) (`self.Damage`)) _asfpschar_2)
    (else
      (`self.K2_DestroyActor`))))

(fn `UserConstructionScript`
  (`parent.UserConstructionScript`))