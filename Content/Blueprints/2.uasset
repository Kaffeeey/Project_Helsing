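; Blueprint actor "2" acts as a damaging hit object, likely a projectile, against Enemy_BP actors.
; On Hit, it casts the other actor to Enemy_BP, subtracts Damage from that enemy's HP, destroys the enemy at zero or below, then destroys itself.
; A failed cast ends the event, so hits on non-enemies leave it alive despite an else branch meant to destroy it.
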(event `self.ReceiveBeginPlay`)

(event `self.ReceiveActorBeginOverlap`
  (params (OtherActor :type "Actor Object Reference")))

(event `self.ReceiveHit`
  (params (MyComp :type "PrimitiveComponent Object Reference") (Other :type "Actor Object Reference") (OtherComp :type "PrimitiveComponent Object Reference") (bSelfMoved :type Boolean) (HitLocation :type "Vector Structure") (HitNormal :type "Vector Structure") (NormalImpulse :type "Vector Structure") (Hit :type "HitResult Structure (by ref)"))
  (bind _asenemy_bp (cast `/Game/Blueprints/Enemy_BP` Other))
  (if (== Other _asenemy_bp)
    (bind _asenemy_bp_2 (cast `/Game/Blueprints/Enemy_BP` Other))
    (bind _output_get (set `/Game/Blueprints/Enemy_BP.HP` (- (`/Game/Blueprints/Enemy_BP.HP` _asenemy_bp_2) (`self.Damage`)) _asenemy_bp_2))
    (if (<= _output_get 0.0)
      (`self.K2_DestroyActor` _asenemy_bp_2))
    (`self.K2_DestroyActor`)
    (else
      (`self.K2_DestroyActor`))))

(fn `UserConstructionScript`)