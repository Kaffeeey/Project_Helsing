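; BP_3D_Menu is a menu actor that hosts a Widget_Master_Menu in the world and moves the player's view between linked menus.
; On BeginPlay it binds to the widget's TransitionToLinkedMenu event and disables its own collision.
; The event's index selects an entry in LinkedMenus, then collision passes from this actor to that menu.
; The player controller's view target blends to the new menu with an ease-in-out transition.
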(event `self.ReceiveBeginPlay`
  (bind _asmaster_menu_widget (cast `/Game/Menu/Widget_Master_Menu` (`WidgetComponent.GetUserWidgetObject` (`self.Widget`))))
  (add `/Game/Menu/Widget_Master_Menu.TransitionToLinkedMenu` _asmaster_menu_widget (delegate `TransitionToLinkedMenu_Event_0`))
  (`self.SetActorEnableCollision` false))

(event `TransitionToLinkedMenu_Event_0`
  (params (MenuIndex :type Integer))
  (if (`KismetArrayLibrary.Array_IsValidIndex` (`self.LinkedMenus`) MenuIndex)
    (`self.TransitionToWidget` (`|GetArrayItem` (`self.LinkedMenus`) MenuIndex))))

(event `TransitionToWidget`
  (params (`New Menu` :type "/Game/Menu/BP_3D_Menu Object Reference"))
  (`self.SetActorEnableCollision` false)
  (`self.SetActorEnableCollision` `New Menu` true)
  (`PlayerController.SetViewTargetWithBlend` (`GameplayStatics.GetPlayerController` 0) `New Menu` 2.0 "VTBlend_EaseInOut" 2.0 false))

(fn `UserConstructionScript`)