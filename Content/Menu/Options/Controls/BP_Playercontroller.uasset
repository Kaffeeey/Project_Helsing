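; Player controller for the options menu that captures a single key press for the controls widget.
; CatchKey stores the requesting controls widget, and the next AnyKey press passes its key to that widget, then clears the reference so only one press is caught.
; Apply, CheckChanges and GetSGAudioSettings are empty stubs, with the first two returning false.
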(event `/Game/Menu/Options/BPI_Menu.CatchKey`
  (params (Widget_Options_Controls1 :type "/Game/Menu/Options/Controls/Widget_Options_Conrols1 Object Reference"))
  (set `self.Widget Options Controls 1` Widget_Options_Controls1))

(event `Key|AnyKey` :consume false
  (params (Key :type "Key Structure"))
  (bind _widget_options_controls_1 (`self.Widget Options Controls 1`))
  (:`Pressed`
    (`/Engine/EditorBlueprintResources/StandardMacros.IsValid` _widget_options_controls_1
      (:`Is Valid`
        (`/Game/Menu/Options/Controls/Widget_Options_Conrols1.AnyKey` _widget_options_controls_1 Key)
        (set `self.Widget Options Controls 1` null)))))

(fn `Apply`
  (returns (Successful :type Boolean))
  (return false))

(fn `CheckChanges`
  (returns (Changes :type Boolean))
  (return false))

(fn `GetSGAudioSettings`
  (returns (SGAudioSettings :type "/Game/SaveFiles/SG_AudioSettings Object Reference"))
  (return null))

(fn `UserConstructionScript`)