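; Actor component for flying AI characters that zeroes gravity and steers the owner around obstacles toward the player.
; CheckForwardArea sphere-traces ahead, caching the hit and writing Obstacle and TargetLocation blackboard keys.
; AlternateRoute tests six axis-offset points around that hit for clearance and reachability, choosing the shortest detour or falling back to the start.
; Separate events move the pawn above the player and check overlapping actors' distance and direction.
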(event `self.ReceiveBeginPlay`
  (bind _ascharacter (cast `Character` (`self.GetOwner`)))
  (bind (_component _valid) (`/Game/AI/FunctionLibrary_AI.GetComponentByClassIfValid` _ascharacter "/Script/Engine.CharacterMovementComponent"))
  (if _valid
    (bind _ascharacter_movement_component (cast `CharacterMovementComponent` _component))
    (set `CharacterMovementComponent.GravityScale` 0.0 _ascharacter_movement_component)))

(event `Fly`
  (bind _ascharacter (cast `Character` (`self.GetOwner`)))
  (bind (_component _valid) (`/Game/AI/FunctionLibrary_AI.GetComponentByClassIfValid` _ascharacter "/Script/Engine.FloatingPawnMovement"))
  (if _valid
    (bind _asfloating_pawn_movement (cast `FloatingPawnMovement` _component))
    (bind _aspawn (cast `Pawn` (`self.GetOwner`)))
    (`|AIMoveTo` _asfloating_pawn_movement _aspawn (+ (`Actor.K2_GetActorLocation` (`GameplayStatics.GetPlayerPawn` 0)) (0.0 0.0 200.0)) null 100.0)))

(event `CheckArea`
  (params (StartPosition :type "Vector Structure") (SphereRadius :type "Float (double-precision)" :default 400.0))
  (bind (_outactors _returnvalue) (`KismetSystemLibrary.SphereOverlapActors` StartPosition SphereRadius (`self.Object Types`)))
  (if _returnvalue
    (for _array_element _outactors
      (`/Game/AI/FunctionLibrary_AI.CheckDistance` (`Actor.K2_GetActorLocation` (`self.GetOwner`)) _array_element)
      (`/Game/AI/FunctionLibrary_AI.CheckDirection` (`self.GetOwner`) _array_element))))

(event `CheckForwardArea`
  (params (Start :type "Vector Structure") (End :type "Vector Structure") (CheckDistance :type "Float (double-precision)" :default 200.0) (Radius :type "Float (double-precision)") (bTraceComplex :type Boolean) (bIgnoreSelf :type Boolean))
  (set `self.StartCheckForward` Start)
  (set `self.EndCheckForward` End)
  (set `self.CheckForwardDistance` CheckDistance)
  (bind (_outhit _returnvalue) (`KismetSystemLibrary.SphereTraceSingleForObjects` :`Start` (`self.StartCheckForward`) :`End` (+ (* (`KismetMathLibrary.GetDirectionUnitVector` (`self.StartCheckForward`) (`self.EndCheckForward`)) (`self.CheckForwardDistance`)) (`self.StartCheckForward`)) :`Radius` Radius :`ObjectTypes` (`self.Object Types`) :`bTraceComplex` bTraceComplex :`bIgnoreSelf` bIgnoreSelf :`TraceColor` (struct :`G` 1.0 :`A` 1.0) :`TraceHitColor` (struct :`R` 1.0 :`A` 1.0) :`DrawTime` 1.0))
  (set `self.LastObstacle` _outhit)
  (`/Game/AI/FunctionLibrary_AI.Set_BB_Key` "NewEnumerator0" (`AIBlueprintHelperLibrary.GetAIController` (`self.GetOwner`)) "Obstacle" _returnvalue)
  (if (not _returnvalue)
    (`/Game/AI/FunctionLibrary_AI.Set_BB_Key` "NewEnumerator9" (`AIBlueprintHelperLibrary.GetAIController` (`self.GetOwner`)) "TargetLocation" false null 0 0.0 0 "None" null (struct) "" (`Actor.K2_GetActorLocation` (`GameplayStatics.GetPlayerPawn` 0)))))

(event `AlternateRoute`
  (params (Start :type "Vector Structure") (Target :type "Vector Structure") (RadiusOfAlternation :type "Float (double-precision)" :default 500.0) (SpheraRadiusAlternatePosition :type "Float (double-precision)" :default 50.0))
  (bind _locationstotest (`self.LocationsToTest`))
  (bind (_bblockinghit _binitialoverlap _time _distance _location _impactpoint _normal _impactnormal _physmat _hitactor) (`GameplayStatics.BreakHitResult` (`self.LastObstacle`)))
  (bind _returnvalue (`AIBlueprintHelperLibrary.GetAIController` (`self.GetOwner`)))
  (set `self.Start` Start)
  (set `self.Target` Target)
  (set `self.Radius Of Alternation` RadiusOfAlternation)
  (set `self.SpheraRadiusAlternatePosition` SpheraRadiusAlternatePosition)
  (set `self.Hit Actor` _hitactor)
  (`KismetArrayLibrary.Array_Add` _locationstotest (+ _location (`KismetMathLibrary.MakeVector` (`self.Radius Of Alternation`))))
  (`KismetArrayLibrary.Array_Add` _locationstotest (+ _location (`KismetMathLibrary.MakeVector` 0.0 (`self.Radius Of Alternation`))))
  (`KismetArrayLibrary.Array_Add` _locationstotest (+ _location (`KismetMathLibrary.MakeVector` 0.0 0.0 (`self.Radius Of Alternation`))))
  (`KismetArrayLibrary.Array_Add` _locationstotest (+ _location (`KismetMathLibrary.MakeVector` (* (`self.Radius Of Alternation`) -1.0))))
  (`KismetArrayLibrary.Array_Add` _locationstotest (+ _location (`KismetMathLibrary.MakeVector` 0.0 (* (`self.Radius Of Alternation`) -1.0))))
  (`KismetArrayLibrary.Array_Add` _locationstotest (+ _location (`KismetMathLibrary.MakeVector` 0.0 0.0 (* (`self.Radius Of Alternation`) -1.0))))
  (for _array_element _locationstotest
    (bind (_returnvalue_2 _testedlocation) (`self.TestPosition` _array_element (`self.SpheraRadiusAlternatePosition`)))
    (if _returnvalue_2
      (bind (_outhit _returnvalue_3) (`KismetSystemLibrary.SphereTraceSingleForObjects` (`self.Start`) _testedlocation 200.0 (`self.Object Types`) false (`self.Actors to Ignore`)))
      (if (not _returnvalue_3)
        (`KismetArrayLibrary.Array_Add` (`self.PossibleLocations`) _testedlocation))))
  (for (_array_element_2 _array_index) (`self.PossibleLocations`)
    (if (== _array_index 0)
      (set `self.LocationIndex` _array_index)
      (bind _returnvalue_4 (+ (`KismetMathLibrary.Vector_Distance` _array_element_2 (`self.Start`)) (`KismetMathLibrary.Vector_Distance` _array_element_2 (`self.Target`))))
      (set `self.Distance` _returnvalue_4)
      (else
        (bind _output_get (set `self.DistanceTemp` _returnvalue_4))
        (if (< _output_get (`self.Distance`))
          (set `self.LocationIndex` _array_index)
          (set `self.Distance` (`self.DistanceTemp`))))))
  (if (> (`KismetArrayLibrary.Array_Length` (`self.PossibleLocations`)) 0)
    (`/Game/AI/FunctionLibrary_AI.Set_BB_Key` "NewEnumerator9" _returnvalue "TargetLocation" false null 0 0.0 0 "None" null (struct) "" (`|GetArrayItem` (`self.PossibleLocations`) (`self.LocationIndex`)))
    (`/Game/AI/FunctionLibrary_AI.Set_BB_Key` "NewEnumerator0" _returnvalue "Obstacle")
    (else
      (`/Game/AI/FunctionLibrary_AI.Set_BB_Key` "NewEnumerator9" _returnvalue "TargetLocation" false null 0 0.0 0 "None" null (struct) "" (`self.Start`)))))

(fn `TestPosition`
  (params (TestLocation :type "Vector Structure") (SphereRadius :type "Float (double-precision)"))
  (returns (ReturnValue :type Boolean) (TestedLocation :type "Vector Structure"))
  (bind (_outactors _returnvalue) (`KismetSystemLibrary.SphereOverlapActors` TestLocation SphereRadius (`self.Object Types`) null (`self.Actors to Ignore`)))
  (return (not _returnvalue) TestLocation))