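; Component that gives a flying AI 3D navigation through the level's NavigationVolume3D, seeding an initial path to the player on BeginPlay.
; FindPath stores an obstacle-aware FlyPath from the owner to a valid target location.
; FollowFlyPath steps through it using AIMoveTo with navmesh pathfinding disabled, toggling the ReachedStep blackboard key around each move.
; After each finished move it recomputes the path but keeps advancing the same index.
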(event `self.ReceiveBeginPlay`
  (bind _returnvalue (`GameplayStatics.GetActorOfClass` "/Script/Navigation3D.NavigationVolume3D"))
  (set `self.NavigationVolume` _returnvalue)
  (`self.FindPath` (`Actor.K2_GetActorLocation` (`GameplayStatics.GetPlayerPawn` 0))))

(event `FindPath`
  (params (TargetLocation :type "Vector Structure"))
  (if (`AIBlueprintHelperLibrary.IsValidAILocation` TargetLocation)
    (bind (_out_path _returnvalue) (`NavigationVolume3D.FindPath` (`self.NavigationVolume`) (`Actor.K2_GetActorLocation` (`self.GetOwner` self)) TargetLocation (`|MakeArray` "ObjectTypeQuery1" "ObjectTypeQuery2" "ObjectTypeQuery8" "ObjectTypeQuery9" "ObjectTypeQuery10" "ObjectTypeQuery11" :!type "EObjectTypeQuery Enum") "/Script/Engine.Actor"))
    (if _returnvalue
      (set `self.FlyPath` _out_path))))

(event `FollowFlyPath`
  (params (AIContoller :type "AIController Object Reference") (AcceptanceRadius :type "Float (double-precision)") (`Target Location` :type "Vector Structure"))
  (set `self.AIContoller` AIContoller)
  (set `self.PathIndex` 0)
  (if (<= (`self.PathIndex`) (`KismetArrayLibrary.Array_LastIndex` (`self.FlyPath`))) :!label _label
    (`/Game/AI/FunctionLibrary_AI.Set_BB_Key` "NewEnumerator0" (`self.AIContoller`) "ReachedStep" true)
    (`AITask_MoveTo.AIMoveTo` (`self.AIContoller`) (`|GetArrayItem` (`self.FlyPath`) (`self.PathIndex`)) null AcceptanceRadius "Enable" "Enable" false false false "Disable"
      (:`OnMoveFinished`
        (`/Engine/EditorBlueprintResources/StandardMacros.IncrementInt` (`self.PathIndex`)
          (:`  `
            (`self.FindPath` `Target Location`)
            (`/Game/AI/FunctionLibrary_AI.Set_BB_Key` "NewEnumerator0" (`self.AIContoller`) "ReachedStep")
            (goto _label)))))))