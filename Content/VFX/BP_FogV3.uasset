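; Volumetric fog actor that fills a sized box using a Niagara particle system with a dynamic fog material.
; The construction script builds render targets and pushes volume, noise, color, shadow and distance-field settings into the material, which feeds the particle.
; A top-down orthographic scene capture of listed actors supplies the height texture, captured on construction and BeginPlay rather than per tick.
; Brush painting appears unfinished: PaintToTexture is never called here and the volume target is unused.
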(event `self.ReceiveBeginPlay`
  (`self.Capture Scene`))

(fn `Capture Scene`
  (`SceneCaptureComponent2D.CaptureScene` (`self.SceneCapture`))
  (return))

(fn `DrawBrush`
  (`|ExecutionSequence`
    (:`then_0`
      (`MaterialInstanceDynamic.SetTextureParameterValue` (`self.BrushMat`) "BrushTex" (`self.BrushTex`)))))

(fn `Height Capture Camera Variables`
  (bind (_returnvalue_x _returnvalue_y _returnvalue_z) (`KismetMathLibrary.BreakVector` (`self.K2_GetActorLocation`)))
  (bind (_volume_size_x _volume_size_y) (`KismetMathLibrary.BreakVector` (`self.Volume Size`)))
  (bind _scenecapture (`self.SceneCapture`))
  (bind (_volume_size_x_2 _volume_size_y_2 _volume_size_z) (`KismetMathLibrary.BreakVector` (`self.Volume Size`)))
  (`SceneComponent.K2_SetWorldLocationAndRotation` _scenecapture (`KismetMathLibrary.MakeVector` _returnvalue_x _returnvalue_y (+ _returnvalue_z (/ _volume_size_z 2.0))) (struct :`Pitch` -90.0 :`Roll` -90.0) false false)
  (set `SceneCaptureComponent2D.OrthoWidth` (`KismetMathLibrary.FMax` _volume_size_x _volume_size_y) _scenecapture)
  (set `SceneCaptureComponent2D.TextureTarget` (`self.Height Capture RT`) _scenecapture)
  (set `SceneCaptureComponent.ShowOnlyActors` (`self.List of Actors used`) _scenecapture))

(fn `Paint To Texture`
  (bind _canvas (`KismetRenderingLibrary.BeginDrawCanvasToRenderTarget` null))
  (`Canvas.K2_DrawMaterial` _canvas (`self.BrushMat`) (0.0 0.0) (0.0 0.0) (0.0 0.0) (1.0 1.0) 0.0 (0.5 0.5)))

(fn `Set Material Variables`
  (bind _mid (`self.MID`))
  (`MaterialInstanceDynamic.SetVectorParameterValue` _mid "VolumeSize" (`KismetMathLibrary.Conv_VectorToLinearColor` (`self.Volume Size`)))
  (`MaterialInstanceDynamic.SetTextureParameterValue` _mid "RT" (`self.Height Capture RT`))
  (`MaterialInstanceDynamic.SetScalarParameterValue` _mid "HeightFalloff" (`self.Height`))
  (`MaterialInstanceDynamic.SetScalarParameterValue` _mid "GlobalExtinctionMultiplier" (`self.Fog Mul`))
  (`MaterialInstanceDynamic.SetScalarParameterValue` _mid "NoiseScale" (`self.Noise Scale`))
  (`MaterialInstanceDynamic.SetScalarParameterValue` _mid "NoisePow" (`self.Noise Pow`))
  (`MaterialInstanceDynamic.SetScalarParameterValue` _mid "Time" (`self.Falling Speed`))
  (`MaterialInstanceDynamic.SetVectorParameterValue` _mid "FogColor" (`self.Fog Color`))
  (`MaterialInstanceDynamic.SetVectorParameterValue` _mid "ShadowColor" (`self.Shadow Color`))
  (`MaterialInstanceDynamic.SetVectorParameterValue` _mid "ExtinctionColor" (`self.Extinction Color`))
  (`MaterialInstanceDynamic.SetScalarParameterValue` _mid "ShadowFalloffDistance" (`self.Shadow Falloff Distance`))
  (`MaterialInstanceDynamic.SetScalarParameterValue` _mid "ShadowDensity" (`self.Shadow Density`))
  (`MaterialInstanceDynamic.SetScalarParameterValue` _mid "ShadowTrace" (`self.Shadow Trace Distance`))
  (`MaterialInstanceDynamic.SetScalarParameterValue` _mid "FogRenderDistance" (`self.Max Render Distance`))
  (if (`self.Distance Field Multiplication`)
    (set `self.Distancefield` 1.0)
    (else
      (set `self.Distancefield` 0.0)))
  (`MaterialInstanceDynamic.SetScalarParameterValue` _mid "DistanceField" (`self.Distancefield`))
  (`MaterialInstanceDynamic.SetScalarParameterValue` _mid "DistanceFieldFalloff" (`self.Distancefield Falloff`)))

(fn `Set Particle Variables`
  (bind _fogparticle (`self.FogParticle`))
  (bind (_volume_size_x _volume_size_y _volume_size_z) (`KismetMathLibrary.BreakVector` (`self.Volume Size`)))
  (`NiagaraComponent.SetVariableMaterial` _fogparticle "FogMID" (`self.MID`))
  (`NiagaraComponent.SetVariableFloat` _fogparticle "VolumeSizeMax" (* (`KismetMathLibrary.FMax` _volume_size_x _volume_size_y _volume_size_z) 1.2)))

(fn `UserConstructionScript`
  (bind _rt_volume_size_x (`self.RT Volume Size X`))
  (bind (_volume_size_x _volume_size_y) (`KismetMathLibrary.BreakVector` (`self.Volume Size`)))
  (bind _returnvalue (`KismetMathLibrary.FTrunc` (`KismetMathLibrary.MultiplyMultiply_FloatFloat` 2.0 (`KismetMathLibrary.Conv_IntToDouble` (`self.Render Target Quality`)))))
  (`BoxComponent.SetBoxExtent` (`self.Visualization`) (/ (`self.Volume Size`) 2.0) true)
  (bind _returnvalue_2 (`KismetMaterialLibrary.CreateDynamicMaterialInstance` "/Game/Materials/M_CHain.M_CHain"))
  (set `self.BrushMat` _returnvalue_2)
  (bind _returnvalue_3 (`KismetMaterialLibrary.CreateDynamicMaterialInstance` "/Game/Materials/M_Fog_V3.M_Fog_V3"))
  (set `self.MID` _returnvalue_3)
  (bind _returnvalue_4 (`KismetRenderingLibrary.CreateRenderTarget2D` _returnvalue _returnvalue))
  (set `self.Height Capture RT` _returnvalue_4)
  (`KismetRenderingLibrary.CreateRenderTargetVolume` _rt_volume_size_x (`KismetMathLibrary.Round` (* _rt_volume_size_x (/ _volume_size_x _volume_size_y))) (`self.RT Volume Size Z`) "RTF_R16f")
  (`self.DrawBrush`)
  (`self.Set Particle Variables`)
  (`self.Set Material Variables`)
  (`self.Height Capture Camera Variables`)
  (`self.Capture Scene`))