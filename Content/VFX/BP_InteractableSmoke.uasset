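; Configurable volumetric smoke volume that shapes an interactive fog material within a box and renders it through a Niagara system.
; The construction script creates fog and height-capture material instances, then pushes shape, noise, falloff, extinction, shadow and color settings to the fog.
; A top-down orthographic scene capture uses a post-process material to write listed actors' heights into a float render target.
; The fog samples that target, with a selectable height method.
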(fn `EditorCapture`
  (`SceneCaptureComponent2D.CaptureScene` (`self.HeightCap`))
  (return))

(fn `HeightCaptureSetup`
  (bind (_returnvalue_x _returnvalue_y _returnvalue_z) (`KismetMathLibrary.BreakVector` (`self.K2_GetActorLocation`)))
  (bind _heightcap (`self.HeightCap`))
  (bind _heightcapmid (`self.HeightcapMID`))
  (bind (_volumesize_x _volumesize_y _volumesize_z) (`KismetMathLibrary.BreakVector` (`self.VolumeSize`)))
  (bind (_volumesize_x_2 _volumesize_y_2 _volumesize_z_2) (`KismetMathLibrary.BreakVector` (`self.VolumeSize`)))
  (set `SceneCaptureComponent2D.PostProcessSettings` (make `PostProcessSettings` :`WeightedBlendables` (make `WeightedBlendables` (`|MakeArray` (make `WeightedBlendable` 1.0 _heightcapmid)))) _heightcap)
  (`MaterialInstanceDynamic.SetScalarParameterValue` _heightcapmid "MaxDepth" _volumesize_z)
  (`SceneComponent.K2_SetWorldLocationAndRotation` _heightcap (`KismetMathLibrary.MakeVector` _returnvalue_x _returnvalue_y (+ _returnvalue_z (/ _volumesize_z 2.0))) (struct :`Pitch` -90.0 :`Roll` -90.0) false false)
  (set `SceneCaptureComponent2D.OrthoWidth` (`KismetMathLibrary.FMax` _volumesize_x_2 _volumesize_y_2 _volumesize_z_2) _heightcap)
  (set `SceneCaptureComponent2D.TextureTarget` (`self.HeightCapture`) _heightcap)
  (set `SceneCaptureComponent.ShowOnlyActors` (`self.Show Only Actors`) _heightcap)
  (`self.EditorCapture`))

(fn `MID Variables`
  (bind _fogmid (`self.FogMID`))
  (`MaterialInstanceDynamic.SetVectorParameterValue` _fogmid "ShapeType" (select `/Game/VFX/E_ShapeType` (`self.ShapeType`) :`NewEnumerator3` (struct :`R` 1.0) :`NewEnumerator5` (struct :`G` 1.0) :`NewEnumerator1` (struct :`B` 1.0) :`NewEnumerator2` (struct :`A` 1.0) :!type "LinearColor Structure"))
  (`MaterialInstanceDynamic.SetVectorParameterValue` _fogmid "VolumeSize" (`KismetMathLibrary.Conv_VectorToLinearColor` (`self.VolumeSize`)))
  (`MaterialInstanceDynamic.SetTextureParameterValue` _fogmid "2D Texture" (`self.2D Texture`))
  (`MaterialInstanceDynamic.SetScalarParameterValue` _fogmid "Falloff" (`self.Falloff`))
  (`MaterialInstanceDynamic.SetScalarParameterValue` _fogmid "Scale" (`self.NoiseScale`))
  (`MaterialInstanceDynamic.SetVectorParameterValue` _fogmid "TimeScale" (`self.TimeScale`))
  (`MaterialInstanceDynamic.SetScalarParameterValue` _fogmid "GlobalExtinction" (`self.GlobalExtinction`))
  (`MaterialInstanceDynamic.SetScalarParameterValue` _fogmid "GlobalHeightFalloff" (`self.Global Height Falloff`))
  (`MaterialInstanceDynamic.SetTextureParameterValue` _fogmid "RT" (`self.HeightCapture`))
  (`MaterialInstanceDynamic.SetVectorParameterValue` _fogmid "HeightMethod" (select `/Game/VFX/E_HeightMethod` (`self.Method`) :`NewEnumerator0` (struct :`R` 1.0) :`NewEnumerator1` (struct :`G` 1.0) :`NewEnumerator3` (struct :`B` 1.0) :`NewEnumerator2` (struct :`A` 1.0) :!type "LinearColor Structure"))
  (`MaterialInstanceDynamic.SetScalarParameterValue` _fogmid "Falloff Power" (`self.Falloff Power`))
  (`MaterialInstanceDynamic.SetScalarParameterValue` _fogmid "Noise Scale" (`self.Noise Scale`))
  (`MaterialInstanceDynamic.SetScalarParameterValue` _fogmid "NoisePow" (`self.NoisePower`))
  (`MaterialInstanceDynamic.SetScalarParameterValue` _fogmid "Timescale" (`self.Noise Rise Speed`))
  (`MaterialInstanceDynamic.SetScalarParameterValue` _fogmid "ShadowDensity" (`self.Shadow Density`))
  (`MaterialInstanceDynamic.SetScalarParameterValue` _fogmid "ShadowFalloffDistance" (`self.Shadow Falloff Distance`))
  (`MaterialInstanceDynamic.SetScalarParameterValue` _fogmid "ShadowTraceDistance" (`self.Shadow Trace Distance`))
  (`MaterialInstanceDynamic.SetVectorParameterValue` _fogmid "FogColor" (`KismetMathLibrary.Conv_ColorToLinearColor` (`self.FogColor`)))
  (`MaterialInstanceDynamic.SetVectorParameterValue` _fogmid "ExtinctionColor" (`KismetMathLibrary.Conv_ColorToLinearColor` (`self.Extinction Color`)))
  (`MaterialInstanceDynamic.SetVectorParameterValue` _fogmid "ShadowColor" (`KismetMathLibrary.Conv_ColorToLinearColor` (`self.Shadow Color`))))

(fn `Niagara Variables`
  (bind _ns_smoke (`self.NS_Smoke`))
  (bind (_volumesize_x _volumesize_y _volumesize_z) (`KismetMathLibrary.BreakVector` (`self.VolumeSize`)))
  (`NiagaraComponent.SetVariableMaterial` _ns_smoke "FogMID" (`self.FogMID`))
  (`NiagaraComponent.SetVariableFloat` _ns_smoke "VolumeSizeMax" (* (`KismetMathLibrary.FMax` _volumesize_x _volumesize_y _volumesize_z) 2.0)))

(fn `UserConstructionScript`
  (`BoxComponent.SetBoxExtent` (`self.Box`) (/ (`self.VolumeSize`) 2.0) true)
  (bind _returnvalue (`KismetMaterialLibrary.CreateDynamicMaterialInstance` "/Game/Materials/Instances/MI_InteractiveFog.MI_InteractiveFog"))
  (set `self.FogMID` _returnvalue)
  (bind _returnvalue_2 (`KismetMaterialLibrary.CreateDynamicMaterialInstance` "/Game/Materials/PP_HeightCapture.PP_HeightCapture"))
  (set `self.HeightcapMID` _returnvalue_2)
  (bind _returnvalue_3 (`KismetRenderingLibrary.CreateRenderTarget2D` 2048 2048 "RTF_R32f"))
  (set `self.HeightCapture` _returnvalue_3)
  (`self.Niagara Variables`)
  (`self.HeightCaptureSetup`)
  (`self.EditorCapture`)
  (`self.MID Variables`))